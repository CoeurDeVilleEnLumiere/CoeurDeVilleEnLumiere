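; Outfit pickup actor that idles on the map with looping bob and spin timelines and a VFX until placed on a character.
; On BeginPlay it takes a random item from GM_Lumiere's pool, then assigns a same-set item to a random empty spawn from OtherSetSpawns.
; Punch drops follow a timeline arc, shortened by a sphere trace hit, with pickup disabled until landing.
; ResetLocAndRot stops animation and undoes hand-item scaling before attachment.
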(event Custom|DropOnPunch
  (params (ForwardCharacterVector :type Vector))
  (bind _returnvalue (Transformation|GetActorLocation))
  ;[1 1 1] Drop Item animation on punch
  (Variables|Drop|SetStartDropLocation _returnvalue)
  (Variables|Drop|SetEndLocation (+ _returnvalue (* ForwardCharacterVector (Variables|/Game/Blueprints/PDA/PDA_Player.PDA_Player_C|GetItemDropForwardForce (Variables|Datas|GetDatasPlayer)))))
  (CallFunction|PunchSphereTrace)
  (Variables|Drop|SetbCanBePickedUp false)
  (bind (_direction _locationprogress _zoffset) (Timeline|Timeline PlayFromStart)
    (:Update
      (Transformation|SetActorLocation (Math|Vector|MakeVector (.NewLocationX (Utilities|CalculateActorLocation _locationprogress _zoffset)) (.NewLocationY (Utilities|CalculateActorLocation _locationprogress _zoffset)) (.NewLocationZ (Utilities|CalculateActorLocation _locationprogress _zoffset))) false false))
    (:Finished
      (Variables|Drop|SetbCanBePickedUp true)
      (CallFunction|ItemonGround))))

(event Custom|ItemSpawned
  ;[1 1 1] Update Number of item already spawned
  (Math|Integer|DecrementInt (Variables|/Game/Core/GM_Lumiere.GM_Lumiere_C|GetNumberOfItems (.AsGM%20Lumiere (Utilities|Casting|CastToGM_Lumiere (Game|GetGameMode))))))

(event Custom|MovingLocation
  ;[1 1 1] Movement in map
  ;;[0.44 0.5941 1] Movement
  (if (Variables|Drop|GetbCanBePickedUp)
    (if (not (Variables|Drop|GetreverseMovement?))
      (bind _alpha (Timeline|MovementLocation Play)
        (:Update
          (Transformation|SetWorldLocation (Variables|Default|GetStaticMesh) (Math|Vector|MakeVector (.NewLocationX (Utilities|NewItemLocation _alpha)) (.NewLocationY (Utilities|NewItemLocation _alpha)) (.NewLocationZ (Utilities|NewItemLocation _alpha))) false false))
        (:Finished
          (if (Variables|Drop|GetbCanBePickedUp)
            (Utilities|FlowControl|FlipFlop
              (:A
                (Variables|Drop|SetreverseMovement? true))
              (:B
                (Variables|Drop|SetreverseMovement? false)))
            (CallFunction|MovingLocation))))
      (else
        (Timeline|MovementLocation Reverse)))))

(event Custom|MovingRotation
  ;[1 1 1] Movement in map
  ;;[1 0.3839 0.284] Rotation
  (if (Variables|Drop|GetbCanBePickedUp)
    (Variables|Default|SetCurrentRotation (Transformation|GetWorldRotation (Variables|Default|GetStaticMesh)))
    (bind _alpha (Timeline|MovementRotation PlayFromStart)
      (:Update
        (Transformation|SetWorldRotation (Variables|Default|GetStaticMesh) (Utilities|NewItemRotation _alpha) false false))
      (:Finished
        (if (Variables|Drop|GetbCanBePickedUp)
          (CallFunction|MovingRotation))))))

(event Custom|StopRotation
  ;[1 1 1] Movement in map
  ;;[1 0.3839 0.284] Rotation
  (bind _alpha (Timeline|MovementRotation Stop)
    (:Update
      (Transformation|SetWorldRotation (Variables|Default|GetStaticMesh) (Utilities|NewItemRotation _alpha) false false))
    (:Finished
      (if (Variables|Drop|GetbCanBePickedUp)
        (CallFunction|MovingRotation)))))

(event Custom|StopMovement
  ;[1 1 1] Movement in map
  ;;[0.44 0.5941 1] Movement
  (bind _alpha (Timeline|MovementLocation Stop)
    (:Update
      (Transformation|SetWorldLocation (Variables|Default|GetStaticMesh) (Math|Vector|MakeVector (.NewLocationX (Utilities|NewItemLocation _alpha)) (.NewLocationY (Utilities|NewItemLocation _alpha)) (.NewLocationZ (Utilities|NewItemLocation _alpha))) false false))
    (:Finished
      (if (Variables|Drop|GetbCanBePickedUp)
        (Utilities|FlowControl|FlipFlop
          (:A
            (Variables|Drop|SetreverseMovement? true))
          (:B
            (Variables|Drop|SetreverseMovement? false)))
        (CallFunction|MovingLocation)))))

(event Custom|ItemOnGround
  ;[1 1 1] Item On Ground
  (Variables|Drop|SetbCanBePickedUp true)
  (Variables|Default|SetInitialLocation (Transformation|GetActorLocation))
  (Variables|Default|SetInitialRotation (Transformation|GetActorRotation))
  (CallFunction|MovingLocation)
  (CallFunction|MovingRotation)
  (Development|SetHiddeninGame (Variables|Default|GetItemVFX) false false))

(event EventBeginPlay
  ;[1 1 1] Begin Play
  (Variables|Ref|SetGmLumiereRef (.AsGM%20Lumiere (Utilities|Casting|CastToGM_Lumiere (Game|GetGameMode))))
  (Components|StaticMesh|SetStaticMesh (Variables|Default|GetStaticMesh) 0)
  (Utilities|FlowControl|DelayUntilNextTick)
  (CallFunction|ItemonGround)
  (Spawn|SpawnItems))

(fn ConstructionScript
  (Class|NiagaraComponent|SetAsset (Variables|Default|GetItemVFX) (Variables|/Game/Blueprints/PDA/PDA_Item.PDA_Item_C|GetItemVFX (Variables|Datas|GetDatasItems)) true))

(fn SpawnFirstRandomItem
  (bind _returnvalue (Game|GetGameMode))
  (bind _staticmesh (Variables|Default|GetStaticMesh))
  (bind _asgm_lumiere (Utilities|Casting|CastToGM_Lumiere _returnvalue))
  (bind _itemscanspawn (Variables|/Game/Core/GM_Lumiere.GM_Lumiere_C|GetItemsCanSpawn _asgm_lumiere))
  (bind _output_get (Variables|Item|SetItem (.OutItem (Utilities|Array|Random _itemscanspawn))))
  (Utilities|Array|RemoveItem _itemscanspawn _output_get)
  (CallFunction|ItemSpawned)
  (Components|StaticMesh|SetStaticMesh (Variables|Default|GetStaticMesh) (.Mesh (Utilities|Struct|BreakS_ItemData (Variables|Item|GetItem))))
  ;[1 1 1] Scale item if is for hand
  (if (== (.SocketType (Utilities|Struct|BreakS_ItemData (Variables|Item|GetItem))) 2)
    (Transformation|SetRelativeScale3D _staticmesh (* (Variables|/Script/Engine.SceneComponent|GetRelativeScale3D _staticmesh) (Variables|Default|GetScaleMultForSmallItem)))))

(fn SpawnSecondSetItem
  (bind _secondsetspawn (Variables|Spawns|GetSecondSetSpawn))
  (bind _staticmesh (Variables|BP_Item_C|GetStaticMesh _secondsetspawn))
  (bind _array_element (Utilities|Array|ForEachLoopwithBreak (Variables|/Game/Core/GM_Lumiere.GM_Lumiere_C|GetItemsCanSpawn (Variables|Ref|GetGmLumiereRef)) :!label _label)
    (:LoopBody
      (LocalVariables|SetSecondItem _array_element)
      (if (Utilities|Enum|Equal(Enum) (.SetType (Utilities|Struct|BreakS_ItemData (Variables|Item|GetItem))) (.SetType (Utilities|Struct|BreakS_ItemData (LocalVariables|GetSecondItem))))
        ;[0.2192 0.4144 1] Set Second Item
        (bind _output_get (Variables|BP_Item_C|SetItem (Variables|Spawns|GetSecondSetSpawn) (LocalVariables|GetSecondItem)))
        (Components|StaticMesh|SetStaticMesh (Variables|BP_Item_C|GetStaticMesh (Variables|Spawns|GetSecondSetSpawn)) (.Mesh (Utilities|Struct|BreakS_ItemData _output_get)))
        (Utilities|Array|RemoveItem (Variables|/Game/Core/GM_Lumiere.GM_Lumiere_C|GetItemsCanSpawn (Variables|Ref|GetGmLumiereRef)) (LocalVariables|GetSecondItem))
        (if (== (.SocketType (Utilities|Struct|BreakS_ItemData (LocalVariables|GetSecondItem))) 2)
          (Transformation|SetRelativeScale3D _staticmesh (* (Variables|/Script/Engine.SceneComponent|GetRelativeScale3D _staticmesh) (Variables|Default|GetScaleMultForSmallItem))))
        (CallFunction|ItemSpawned)
        (goto _label Break)))))

(fn SpawnItems
  (if (> (Variables|/Game/Core/GM_Lumiere.GM_Lumiere_C|GetNumberOfItems (Variables|Ref|GetGmLumiereRef)) 0)
    ;[0.2417 0.53 1] Check Item is null
    (if (Utilities|Enum|Equal(Enum) (.Name (Utilities|Struct|BreakS_ItemData (Variables|Item|GetItem))) "Null")
      (Spawn|SpawnFirstRandomItem)
      (Spawn|ChooseSecondSpawn))))

(fn ChooseSecondSpawn
  (bind _othersetspawns (Variables|Spawns|GetOtherSetSpawns))
  (if (Utilities|Array|IsNotEmpty _othersetspawns)
    (bind _output_get (Variables|Spawns|SetSecondSetSpawn (.OutItem (Utilities|Array|Random _othersetspawns))))
    (if (Utilities|Enum|Equal(Enum) (.Name (Utilities|Struct|BreakS_ItemData (Variables|BP_Item_C|GetItem _output_get))) "Null")
      (Spawn|SpawnSecondSetItem)
      (else
        (Utilities|Array|RemoveItem (Variables|Spawns|GetOtherSetSpawns) (Variables|Spawns|GetSecondSetSpawn))
        (Spawn|ChooseSecondSpawn)))))

(fn PunchSphereTrace
  (bind (_outhit _returnvalue) (Collision|SphereTraceForObjects (Variables|Drop|GetStartDropLocation) (Variables|Drop|GetEndLocation) (Components|Sphere|GetScaledSphereRadius (Variables|Default|GetSphere)) (Utilities|Array|MakeArray "ObjectTypeQuery1" "ObjectTypeQuery2") false 0 "None"))
  (if _returnvalue
    (Variables|Drop|SetEndLocation (.Location (Collision|BreakHitResult _outhit))))
  (return))

(fn ResetLocandRot
  (bind _staticmesh (Variables|Default|GetStaticMesh))
  ;[1 0.6428 0.3431] Stop and reset rotation and location before putting on the character
  (Variables|Drop|SetbCanBePickedUp false)
  (CallFunction|StopMovement)
  (CallFunction|StopRotation)
  (Transformation|SetWorldLocationAndRotation (Variables|Default|GetStaticMesh) (Variables|Default|GetInitialLocation) (Variables|Default|GetInitialRotation) false false)
  (Development|SetHiddeninGame (Variables|Default|GetItemVFX) true false)
  ;[1 0.4538 0.404] Remove scaling before putting on character if hand item
  (if (== (.SocketType (Utilities|Struct|BreakS_ItemData (Variables|Item|GetItem))) 2)
    (Transformation|SetRelativeScale3D _staticmesh (/ (Variables|/Script/Engine.SceneComponent|GetRelativeScale3D _staticmesh) (Variables|Default|GetScaleMultForSmallItem)))))