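; Roaming AI camera pawn that takes timed pictures during a round and scores players caught in frame.
; On game start it wanders to random navmesh points between randomized delays computed from round time, then stops, flickers its spotlight, flashes and triggers BP_PictureCamera capture.
; Activating nested Center, Side and BarelyVisible volumes reports players' screen position and foreground, plus sound and VFX.
; Pickable items are hidden during capture; exhausted delays end the game.
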(event OnComponentActivated(BarelyVisible)
  (params (Component :type Actor%20Component%20Object%20Reference) (bReset :type Boolean))
  (bind _returnvalue (Game|Player|GetPlayerPawn 1))
  (bind _returnvalue_2 (Game|Player|GetPlayerPawn 0))
  (bind _barelyvisible (Variables|Default|GetBarelyVisible))
  (bind _overlappingactors (Collision|GetOverlappingActors _barelyvisible "/Game/Core/BP_Character.BP_Character_C" :!class /Script/Engine.PrimitiveComponent))
  ;[1 1 1] Box Picture Overlap
  (for _array_element _overlappingactors
    (bind _character (Class|BPIRef|ReftoCharacter(Message) _array_element))
    (Default|PositiononScreen _character "NewEnumerator2")
    ;;[0 1 0.1382] Sound Effect if player here
    (Audio|PlaySound2D "/Game/Audio/SoundEffects/Cues/Player/SC_SetPoseWow.SC_SetPoseWow" 1.0 1.0 0.0 0 0)
    (Variables|Default|SetPlayerInPicture true)
    (switch int (Variables|/Game/Core/BP_Character.BP_Character_C|GetPlayerIndex _character)
      (:0
        (Class|NiagaraComponent|SetAsset (Variables|Default|GetPictureVFX) (Variables|/Game/Blueprints/PDA/PDA_MovingCamera.PDA_MovingCamera_C|GetVFXPicP1 (Variables|Data|GetDatasMovingCamera)) true))
      (:1
        (Class|NiagaraComponent|SetAsset (Variables|Default|GetPictureVFX) (Variables|/Game/Blueprints/PDA/PDA_MovingCamera.PDA_MovingCamera_C|GetVFXPicP2 (Variables|Data|GetDatasMovingCamera)) true))))
  (if (>= (Utilities|Array|Length _overlappingactors) 2)
    ;;[0.2902 0.6118 1] Foreground Score
    (Variables|Default|Set2PlayerInPic true)
    (if (< (.x (Transformation|GetActorLocation _returnvalue_2)) (.x (Transformation|GetActorLocation _returnvalue)))
      (bind _character_2 (Class|BPIRef|ReftoCharacter(Message) _returnvalue_2))
      (Default|ForegroundScore _character_2)
      (else
        (bind _character_3 (Class|BPIRef|ReftoCharacter(Message) _returnvalue))
        (Default|ForegroundScore _character_3)))
    (else
      (Variables|Default|Set2PlayerInPic false)
      (bind _character_4 (Class|BPIRef|ReftoCharacter(Message) (Utilities|Array|Get(acopy) _overlappingactors)))
      (Utilities|IsValid _character_4
        (:Is%20Valid
          (Default|ForegroundScore _character_4))))))

(event OnComponentActivated(Side)
  (params (Component :type Actor%20Component%20Object%20Reference) (bReset :type Boolean))
  ;[1 1 1] Box Picture Overlap
  ;;[1 0.7041 0.2686] Side
  (for _array_element (Collision|GetOverlappingActors (Variables|Default|GetSide) "/Game/Core/BP_Character.BP_Character_C" :!class /Script/Engine.PrimitiveComponent)
    (Development|PrintString "Side")
    (bind _character (Class|BPIRef|ReftoCharacter(Message) _array_element))
    (Default|PositiononScreen _character "NewEnumerator1")))

(event OnComponentActivated(Center)
  (params (Component :type Actor%20Component%20Object%20Reference) (bReset :type Boolean))
  ;[1 1 1] Box Picture Overlap
  ;;[0.4203 1 0.3757] Center
  (for _array_element (Collision|GetOverlappingActors (Variables|Default|GetCenter) "/Game/Core/BP_Character.BP_Character_C" :!class /Script/Engine.PrimitiveComponent)
    (bind _character (Class|BPIRef|ReftoCharacter(Message) _array_element))
    (Default|PositiononScreen _character "NewEnumerator0")))

(event Custom|Move
  ;[1 1 1] Frame Moving
  (Rendering|SetVisibility (Variables|Default|GetSpotLight) false false)
  (Components|Activation|Deactivate (Variables|Default|GetBarelyVisible))
  (Components|Activation|Deactivate (Variables|Default|GetSide))
  (Components|Activation|Deactivate (Variables|Default|GetCenter))
  (bind _output_get (Variables|Movement|SetRandomLocation (.RandomLocation (AI|Navigation|GetRandomReachablePointinRadius (Transformation|GetActorLocation) 9e+02 0 0))))
  (AI|AIMoveTo self _output_get 0 2e+01 false
    (:OnSuccess
      _)
    (:OnFail
      _))
  (if (not (Variables|Default|GetbTakePicture))
    (CallFunction|Move)))

(event Custom|GameStart_Event
  ;[1 1 1] On  Game Start
  (Rendering|SetVisibility (Variables|Default|GetCameraWidget) true false)
  (CallFunction|WaitforPicture))

(event Custom|WaitForPicture
  (bind _delaybetweenpics (Variables|BetweenPic|GetDelayBetweenPics))
  (bind _delayindex (Variables|BetweenPic|GetDelayIndex))
  (bind _output (Utilities|Array|Get(acopy) _delaybetweenpics _delayindex))
  ;[1 1 1] Move
  (Default|CallMoveAfterPicture)
  (Variables|Default|SetbTakePicture false)
  (CallFunction|Move)
  ;[1 1 1] Time to wait before taking picture
  (if (not (<= _output 0.0))
    (Utilities|FlowControl|Delay _output)
    (Math|Integer|IncrementInt (Variables|BetweenPic|GetDelayIndex)
      (:%20%20
        ;[1 1 1] Take Picture
        (CallFunction|TakePicture)))
    (else
      (Default|EndOfGame (.AsGM%20Lumiere (Utilities|Casting|CastToGM_Lumiere (Game|GetGameMode)))))))

(event Custom|TakePicture
  (bind _picturevfx (Variables|Default|GetPictureVFX))
  ;[1 1 1] Picture time
  (Default|CallPictureStopMoving)
  (Variables|Default|SetbTakePicture true)
  ;;[0.2918 0.6105 1] In position for picture
  (CallFunction|FlickingSpotLight)
  (Class|NavMovementComponent|StopActiveMovement (Variables|Default|GetFloatingPawnMovement))
  (Utilities|FlowControl|Delay (Variables|/Game/Blueprints/PDA/PDA_MovingCamera.PDA_MovingCamera_C|GetDelayBeforeFlash (Variables|Data|GetDatasMovingCamera)))
  (CallFunction|HideItemsinFrame true)
  ;;[0 1 0.1382] Simple click of picture
  (Audio|PlaySound2D "/Game/Audio/SoundEffects/Picture/camera-appareil-photo-prise-shot-346097.camera-appareil-photo-prise-shot-346097" 3.0 1.0 0.2 0 0)
  ;;[0.2902 0.6118 1] Take Picture
  (bind _returnvalue (UserInterface|CreateWidget "/Game/Blueprints/Widget/WBP_Flash.WBP_Flash_C"))
  (UserInterface|Viewport|AddtoViewport _returnvalue 0)
  (Default|CaptureImage (Variables|Ref|GetPictureCameraRef))
  (Score|ComputeScore)
  (CallFunction|HideItemsinFrame false)
  ;;[0.2918 0.6105 1] Show Picture
  (Utilities|FlowControl|Delay (Variables|/Game/Blueprints/PDA/PDA_MovingCamera.PDA_MovingCamera_C|GetDelayAfterPicture (Variables|Data|GetDatasMovingCamera)))
  ;[0.2918 0.6105 1] Move Again
  (CallFunction|WaitforPicture)
  ;[1 1 1] VFX effect if in pic
  (if (Variables|Default|GetPlayerInPicture)
    (if (Variables|Default|Get2PlayerInPic)
      (Class|NiagaraComponent|SetAsset _picturevfx (Variables|/Game/Blueprints/PDA/PDA_MovingCamera.PDA_MovingCamera_C|GetVFXPicP1 (Variables|Data|GetDatasMovingCamera)) true)
      (Components|Activation|Activate _picturevfx true)
      (Components|Activation|Activate (Variables|Default|GetPictureVFXSecondary) true)
      (else
        (Components|Activation|Activate (Variables|Default|GetPictureVFX) true)
        (Variables|Default|SetPlayerInPicture false)))))

(event Custom|FlickingSpotLight
  ;[1 1 1] Flashing Light Before Picture is taken
  (if (Variables|Default|GetbTakePicture)
    (Utilities|ForLoopwithDelay 0 4 0.5
      (:Loop%20Body
        (Utilities|FlowControl|FlipFlop
          (:A
            (Rendering|SetVisibility (Variables|Default|GetSpotLight) true false))
          (:B
            (Rendering|SetVisibility (Variables|Default|GetSpotLight) false false))))
      (:Completed
        (Rendering|SetVisibility (Variables|Default|GetSpotLight) true false)))))

(event Custom|Hide%20Items%20in%20Frame
  (params (Hide :type Boolean))
  ;[0.5165 0.3972 1] Hide Items in Frame
  (for _array_element (Collision|GetOverlappingActors (Variables|Default|GetBarelyVisible) "/Game/Blueprints/Ouftit/BP_Item.BP_Item_C" :!class /Script/Engine.PrimitiveComponent)
    (bind _asbp_item (Utilities|Casting|CastToBP_Item _array_element))
    (if (Variables|/Game/Blueprints/Ouftit/BP_Item.BP_Item_C|GetbCanBePickedUp _asbp_item)
      (Rendering|SetActorHiddenInGame _array_element Hide))))

(event EventBeginPlay
  ;[1 1 1] Begin Play
  (Rendering|SetVisibility (Variables|Default|GetCameraWidget) false false)
  (Variables|/Script/Engine.FloatingPawnMovement|SetMaxSpeed (Variables|Default|GetFloatingPawnMovement) (Variables|/Game/Blueprints/PDA/PDA_MovingCamera.PDA_MovingCamera_C|GetSpeed (Variables|Data|GetDatasMovingCamera)))
  (bind _returnvalue (Actor|GetActorOfClass "/Game/Blueprints/Camera/BP_PictureCamera.BP_PictureCamera_C"))
  (Variables|Ref|SetPictureCameraRef _returnvalue)
  (CallFunction|SetDelayBetweenPic)
  (bind _aswbp_camera_video (Utilities|Casting|CastToWBP_CameraVideo (UserInterface|GetWidget (Variables|Default|GetCameraWidget))))
  (Variables|Ref|SetWBP_CameraVideo _aswbp_camera_video)
  ;[1 1 1] On  Game Start
  (EventDispatchers|AssignGameStart (.AsGM%20Lumiere (Utilities|Casting|CastToGM_Lumiere (Game|GetGameMode))) (delegate Custom|GameStart_Event)))

(fn ConstructionScript)

(fn SetDelayBetweenPic
  (bind _datasmovingcamera (Variables|Data|GetDatasMovingCamera))
  ;[0.375 0.4466 1] Round Time without time of pictures
  (bind _output_get (Variables|RoundTimeWithoutPicsTime|SetTotalDelayPerPicture (+ (Variables|/Game/Blueprints/PDA/PDA_MovingCamera.PDA_MovingCamera_C|GetDelayAfterPicture _datasmovingcamera) (Variables|/Game/Blueprints/PDA/PDA_MovingCamera.PDA_MovingCamera_C|GetDelayBeforeShowingPic _datasmovingcamera) (Variables|/Game/Blueprints/PDA/PDA_MovingCamera.PDA_MovingCamera_C|GetDelayBeforeFlash _datasmovingcamera))))
  (bind _output_get_2 (Variables|RoundTimeWithoutPicsTime|SetFixedTimePerRound (* _output_get (Variables|/Game/Blueprints/PDA/PDA_Round.PDA_Round_C|GetPictureNumbers (Variables|Data|GetDatasRound)))))
  (Variables|RoundTimewithoutpicstime|SetRoundTime (- (Variables|/Game/Blueprints/PDA/PDA_Round.PDA_Round_C|GetRoundTime (Variables|Data|GetDatasRound)) _output_get_2))
  ;[0.3146 0.3871 1] Max movement delay between pic
  (Variables|Movement|Delay|SetMaxPicDelay (/ (Variables|RoundTimewithoutpicstime|GetRoundTime) (Variables|/Game/Blueprints/PDA/PDA_Round.PDA_Round_C|GetPictureNumbers (Variables|Data|GetDatasRound))))
  ;[0.5412 1 0.6982] All Pictures except -1
  (for _index (range 0 (- (Variables|/Game/Blueprints/PDA/PDA_Round.PDA_Round_C|GetPictureNumbers (Variables|Data|GetDatasRound)) 1))
    (bind _output_get_3 (Variables|Movement|Delay|SetRandomDelay (Math|Random|RandomFloatinRange (/ (* (Variables|/Game/Blueprints/PDA/PDA_MovingCamera.PDA_MovingCamera_C|GetMinPercentageTimeBetweenPic (Variables|Data|GetDatasMovingCamera)) (Variables|RoundTimewithoutpicstime|GetRoundTime)) 1e+02) (Variables|Movement|Delay|GetMaxPicDelay))))
    (Utilities|Array|SetArrayElem (Variables|BetweenPic|GetDelayBetweenPics) _index _output_get_3 true)
    (Variables|BetweenPic|SetDelayBetweenPictureWithoutLast (+ _output_get_3 (Variables|BetweenPic|GetDelayBetweenPictureWithoutLast))))
  ;[1 0.439 0.5799] Last Pic
  (Utilities|Array|SetArrayElem (Variables|BetweenPic|GetDelayBetweenPics) (Variables|/Game/Blueprints/PDA/PDA_Round.PDA_Round_C|GetPictureNumbers (Variables|Data|GetDatasRound)) (- (Variables|RoundTimewithoutpicstime|GetRoundTime) (Variables|BetweenPic|GetDelayBetweenPictureWithoutLast)) true))

(fn ComputeScore
  (Components|Activation|Activate (Variables|Default|GetBarelyVisible) false)
  (Components|Activation|Activate (Variables|Default|GetSide) false)
  (Components|Activation|Activate (Variables|Default|GetCenter) false))

(fn IsPlayerinPicture
  (params (PlayerPawn :type Pawn%20Object%20Reference) (PlayerId :type Integer))
  (bind _returnvalue (Game|GetPlayerController PlayerId))
  (bind _returnvalue_2 (Transformation|GetActorLocation PlayerPawn))
  (bind _returnvalue_3 (Game|GetPlayerController PlayerId))
  (bind _self self)
  (bind _screenposition (Class|GameplayStatics|ProjectWorldtoScreen _returnvalue _returnvalue_2 false))
  (bind _returnvalue_4 (Pawn|GetNavAgentLocation _self))
  (bind _screenposition_2 (Class|GameplayStatics|ProjectWorldtoScreen _returnvalue_3 _returnvalue_4 false))
  ;[1 0 0] TODO calcul position joueur par rapport au widget de caméra
  (bind _sizeofcamera (Default|GetSize (Variables|Ref|GetWBP_CameraVideo)))
  (if (not (Math|Boolean|ORBoolean (>= (- (.x _screenposition) (/ (.x _sizeofcamera) 2.0)) (.x _screenposition_2)) (<= (+ (+ (.x _screenposition) (/ (.x _sizeofcamera) 2.0)) 5e+01) (.x _screenposition_2)) (>= (- (.y _screenposition) (/ (.y _sizeofcamera) 2.0)) (.y _screenposition_2)) (<= (+ (+ (.y _screenposition) (/ (.y _sizeofcamera) 2.0)) 5e+01) (.y _screenposition_2))))
    (Development|PrintString (Utilities|String|Append "Player " (Utilities|String|ToString(Integer) PlayerId) " is in the Picture"))
    (return true)
    (else
      (Development|PrintString (Utilities|String|Append "Player " (Utilities|String|ToString(Integer) PlayerId) " is Hidden"))
      (return false))))