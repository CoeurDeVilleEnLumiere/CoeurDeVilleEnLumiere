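; In-game photo camera that captures the scene, shows each shot in a WBP_Picture widget after a delay, and tracks it for saving.
; Each shot renders into two fresh targets, one for display and HDR export, one RGBA8 for PNG; SaveAllPictures writes both to disk.
; Contrast, saturation and gamma from GI_Lumiere grade the display capture only.
; Later adjustments unpause the game for one tick, then pause it again.
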(event Custom|SetGamma
  (params (gamma :type Float%20%28double-precision%29) (beginPlay :type Boolean))
  (bind _returnvalue (Game|GetGameInstance))
  (bind _asgi_lumiere (Utilities|Casting|CastToGI_Lumiere _returnvalue))
  (Variables|/Script/Engine.SceneCaptureComponent2D|SetPostProcessSettings (Variables|Default|GetSceneCaptureComponent2D%20) (Utilities|Struct|MakePostProcessSettings (Math|Vector4|MakeVector4 1.0 1.0 1.0 (Variables|/Game/Core/GI_Lumiere.GI_Lumiere_C|GetCameraSaturation _asgi_lumiere)) (Math|Vector4|MakeVector4 1.0 1.0 1.0 (Variables|/Game/Core/GI_Lumiere.GI_Lumiere_C|GetCameraContrast _asgi_lumiere)) (Math|Vector4|MakeVector4 1.0 1.0 1.0 gamma)))
  (if (not beginPlay)
    (Game|SetGamePaused false)
    (Utilities|FlowControl|DelayUntilNextTick)
    (Game|SetGamePaused true)))

(event Custom|SetContrast
  (params (contrast :type Float%20%28double-precision%29) (beginPlay :type Boolean))
  (bind _returnvalue (Game|GetGameInstance))
  (bind _asgi_lumiere (Utilities|Casting|CastToGI_Lumiere _returnvalue))
  (Variables|/Script/Engine.SceneCaptureComponent2D|SetPostProcessSettings (Variables|Default|GetSceneCaptureComponent2D%20) (Utilities|Struct|MakePostProcessSettings (Math|Vector4|MakeVector4 1.0 1.0 1.0 (Variables|/Game/Core/GI_Lumiere.GI_Lumiere_C|GetCameraSaturation _asgi_lumiere)) (Math|Vector4|MakeVector4 1.0 1.0 1.0 contrast) (Math|Vector4|MakeVector4 1.0 1.0 1.0 (Variables|/Game/Core/GI_Lumiere.GI_Lumiere_C|GetCameraGamma _asgi_lumiere))))
  (if (not beginPlay)
    (Game|SetGamePaused false)
    (Utilities|FlowControl|DelayUntilNextTick)
    (Game|SetGamePaused true)))

(event Custom|CaptureImage
  (bind _returnvalue (Rendering|CreateRenderTarget2D 1920 1080 "RTF_RGBA8"))
  (Variables|/Script/Engine.SceneCaptureComponent2D|SetTextureTarget (Variables|Default|GetSceneCaptureForExport) _returnvalue)
  (bind _returnvalue_2 (Rendering|CreateRenderTarget2D 1920 1080 "RTF_RGBA16f"))
  (bind _output_get (Variables|/Script/Engine.SceneCaptureComponent2D|SetTextureTarget (Variables|Default|GetSceneCaptureComponent2D%20) _returnvalue_2))
  (bind _returnvalue_3 (UserInterface|CreateWidget "/Game/Blueprints/Widget/WBP_Picture.WBP_Picture_C" 0 _output_get))
  (Variables|Ref|SetPictureWidgetRef _returnvalue_3)
  (Rendering|SceneCapture|CaptureScene (Variables|Default|GetSceneCaptureComponent2D%20) :!class /Script/Engine.SceneCaptureComponent2D)
  (Rendering|SceneCapture|CaptureScene (Variables|Default|GetSceneCaptureForExport) :!class /Script/Engine.SceneCaptureComponent2D)
  ;[0.1374 1 0.3179] Swoosh of picture appearing on screen
  (Audio|PlaySound2D 0 1.0 1.0 0.0 0 0)
  (CallFunction|SavePictureSpecification)
  (Utilities|FlowControl|Delay (Variables|/Game/Blueprints/PDA/PDA_MovingCamera.PDA_MovingCamera_C|GetDelayBeforeShowingPic (Variables|Default|GetDatasMovingCamera)))
  (UserInterface|Viewport|AddtoViewport (Variables|Ref|GetPictureWidgetRef) 0))

(event Custom|SetSaturation
  (params (saturation :type Float%20%28double-precision%29) (beginPlay :type Boolean))
  (bind _returnvalue (Game|GetGameInstance))
  (bind _asgi_lumiere (Utilities|Casting|CastToGI_Lumiere _returnvalue))
  (Variables|/Script/Engine.SceneCaptureComponent2D|SetPostProcessSettings (Variables|Default|GetSceneCaptureComponent2D%20) (Utilities|Struct|MakePostProcessSettings (Math|Vector4|MakeVector4 1.0 1.0 1.0 saturation) (Math|Vector4|MakeVector4 1.0 1.0 1.0 (Variables|/Game/Core/GI_Lumiere.GI_Lumiere_C|GetCameraContrast _asgi_lumiere)) (Math|Vector4|MakeVector4 1.0 1.0 1.0 (Variables|/Game/Core/GI_Lumiere.GI_Lumiere_C|GetCameraGamma _asgi_lumiere))))
  (if (not beginPlay)
    (Game|SetGamePaused false)
    (Utilities|FlowControl|DelayUntilNextTick)
    (Game|SetGamePaused true)))

(event EventBeginPlay
  (Variables|Ref|SetGI_LumiereRef (.AsGI%20Lumiere (Utilities|Casting|CastToGI_Lumiere (Game|GetGameInstance))))
  (bind _asgi_lumiere (Utilities|Casting|CastToGI_Lumiere (Game|GetGameInstance)))
  (CallFunction|SetContrast (Variables|/Game/Core/GI_Lumiere.GI_Lumiere_C|GetCameraContrast _asgi_lumiere) true)
  (CallFunction|SetSaturation (Variables|/Game/Core/GI_Lumiere.GI_Lumiere_C|GetCameraSaturation _asgi_lumiere) true)
  (CallFunction|SetGamma (Variables|/Game/Core/GI_Lumiere.GI_Lumiere_C|GetCameraGamma _asgi_lumiere) true))

(fn ConstructionScript)

(fn SaveAllPictures
  (for (_array_element _array_index) (Variables|Default|GetAllPictures)
    (Rendering|ExportRenderTarget _array_element (Variables|/Game/Core/GI_Lumiere.GI_Lumiere_C|GetHDRDirectoryPath (Variables|Ref|GetGI_LumiereRef)) (Utilities|Array|Get(acopy) (Variables|Default|GetAllPicturesName) _array_index)))
  (for (_array_element_2 _array_index_2) (Variables|Default|GetAllPicturesToExport)
    (Class|ImageWriteBlueprintLibrary|ExporttoDisk _array_element_2 (Utilities|String|Append (Variables|/Game/Core/GI_Lumiere.GI_Lumiere_C|GetPNGDirectoryPath (Variables|Ref|GetGI_LumiereRef)) "/" (Utilities|Array|Get(acopy) (Variables|Default|GetAllPicturesName) _array_index_2)) (Utilities|Struct|MakeImageWriteOptions "PNG" "(null).None" 0 true true))))

(fn SavePictureSpecification
  (bind _gi_lumiereref (Variables|Ref|GetGI_LumiereRef))
  (bind _pictureindex (Variables|/Game/Core/GI_Lumiere.GI_Lumiere_C|GetPictureIndex _gi_lumiereref))
  (bind _returnvalue (Utilities|String|ToString(Integer) _pictureindex))
  (bind _returnvalue_2 (Utilities|String|Append "Photo" _returnvalue))
  (Utilities|Array|Add (Variables|Default|GetAllPicturesToExport) (Variables|/Script/Engine.SceneCaptureComponent2D|GetTextureTarget (Variables|Default|GetSceneCaptureForExport)))
  (Utilities|Array|Add (Variables|Default|GetAllPictures) (Variables|/Script/Engine.SceneCaptureComponent2D|GetTextureTarget (Variables|Default|GetSceneCaptureComponent2D%20)))
  (Default|AddPicture (Variables|Ref|GetGI_LumiereRef) _returnvalue_2)
  (Utilities|Array|Add (Variables|Default|GetAllPicturesName) _returnvalue_2)
  (Default|IncrementPictureCounter (Variables|Ref|GetGI_LumiereRef)))