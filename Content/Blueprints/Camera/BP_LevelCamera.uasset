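; Level camera that becomes the player's view target on BeginPlay and applies the saturation, contrast and gamma stored in GI_Lumiere.
; Each setter rebuilds the camera's post-process settings from its new value plus the other two read from the game instance.
; Calls made outside BeginPlay unpause the game for one tick, then pause it again, presumably to refresh the image while paused.
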(event Custom|SetGamma
  (params (gamma :type Float%20%28double-precision%29) (fromBeginPlay :type Boolean))
  (bind _returnvalue (Game|GetGameInstance))
  (bind _asgi_lumiere (Utilities|Casting|CastToGI_Lumiere _returnvalue))
  (Variables|/Script/Engine.CameraComponent|SetPostProcessSettings (Variables|CameraActor|GetCameraComponent) (Utilities|Struct|MakePostProcessSettings (Math|Vector4|MakeVector4 1.0 1.0 1.0 (Variables|/Game/Core/GI_Lumiere.GI_Lumiere_C|GetCameraSaturation _asgi_lumiere)) (Math|Vector4|MakeVector4 1.0 1.0 1.0 (Variables|/Game/Core/GI_Lumiere.GI_Lumiere_C|GetCameraContrast _asgi_lumiere)) (Math|Vector4|MakeVector4 1.0 1.0 1.0 gamma)))
  (if (not fromBeginPlay)
    (Game|SetGamePaused false)
    (Utilities|FlowControl|DelayUntilNextTick)
    (Game|SetGamePaused true)))

(event Custom|SetContrast
  (params (contrast :type Float%20%28double-precision%29) (fromBeginPlay :type Boolean))
  (bind _returnvalue (Game|GetGameInstance))
  (bind _asgi_lumiere (Utilities|Casting|CastToGI_Lumiere _returnvalue))
  (Variables|/Script/Engine.CameraComponent|SetPostProcessSettings (Variables|CameraActor|GetCameraComponent) (Utilities|Struct|MakePostProcessSettings (Math|Vector4|MakeVector4 1.0 1.0 1.0 (Variables|/Game/Core/GI_Lumiere.GI_Lumiere_C|GetCameraSaturation _asgi_lumiere)) (Math|Vector4|MakeVector4 1.0 1.0 1.0 contrast) (Math|Vector4|MakeVector4 1.0 1.0 1.0 (Variables|/Game/Core/GI_Lumiere.GI_Lumiere_C|GetCameraGamma _asgi_lumiere))))
  (if (not fromBeginPlay)
    (Game|SetGamePaused false)
    (Utilities|FlowControl|DelayUntilNextTick)
    (Game|SetGamePaused true)))

(event Custom|SetSaturation
  (params (saturation :type Float%20%28double-precision%29) (fromBeginPlay :type Boolean))
  (bind _returnvalue (Game|GetGameInstance))
  (bind _asgi_lumiere (Utilities|Casting|CastToGI_Lumiere _returnvalue))
  (Variables|/Script/Engine.CameraComponent|SetPostProcessSettings (Variables|CameraActor|GetCameraComponent) (Utilities|Struct|MakePostProcessSettings (Math|Vector4|MakeVector4 1.0 1.0 1.0 saturation) (Math|Vector4|MakeVector4 1.0 1.0 1.0 (Variables|/Game/Core/GI_Lumiere.GI_Lumiere_C|GetCameraContrast _asgi_lumiere)) (Math|Vector4|MakeVector4 1.0 1.0 1.0 (Variables|/Game/Core/GI_Lumiere.GI_Lumiere_C|GetCameraGamma _asgi_lumiere))))
  (if (not fromBeginPlay)
    (Game|SetGamePaused false)
    (Utilities|FlowControl|DelayUntilNextTick)
    (Game|SetGamePaused true)))

(event EventBeginPlay
  (Game|Player|SetViewTargetwithBlend (Game|GetPlayerController 0) self 0.0 "VTBlend_Linear" 0.0 false)
  (bind _asgi_lumiere (Utilities|Casting|CastToGI_Lumiere (Game|GetGameInstance)))
  (CallFunction|SetContrast (Variables|/Game/Core/GI_Lumiere.GI_Lumiere_C|GetCameraContrast _asgi_lumiere) true)
  (CallFunction|SetSaturation (Variables|/Game/Core/GI_Lumiere.GI_Lumiere_C|GetCameraSaturation _asgi_lumiere) true)
  (CallFunction|SetGamma (Variables|/Game/Core/GI_Lumiere.GI_Lumiere_C|GetCameraGamma _asgi_lumiere) true))

(fn ConstructionScript)