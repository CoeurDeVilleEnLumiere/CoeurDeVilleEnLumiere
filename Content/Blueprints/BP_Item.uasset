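; BP_Item is an item spawn point that randomly receives items in matching set pairs from GM_Lumiere's shared pool.
; On BeginPlay it clears its mesh, waits a tick, then, if still empty and items remain, takes a random pool item.
; It recursively seeks an empty point in OtherSetSpawns and assigns it the first pooled item of the same SetType.
; Each assignment updates the mesh and game mode's pool and count.
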(event Custom|ChooseSecondSpawn
  (bind _othersetspawns (Variables|Spawns|GetOtherSetSpawns))
  ;[1 1 1] Second Spawn Logic
  (if (Utilities|Array|IsNotEmpty _othersetspawns)
    (bind _output_get (Variables|Spawns|SetSecondSetSpawn (.OutItem (Utilities|Array|Random _othersetspawns))))
    (if (Utilities|Enum|Equal(Enum) (.Name (Utilities|Struct|BreakS_ItemData (Variables|BP_Item_C|GetItem _output_get))) "Null")
      (CallFunction|SpawnSecondSetItem)
      (else
        (Utilities|Array|RemoveItem (Variables|Spawns|GetOtherSetSpawns) (Variables|Spawns|GetSecondSetSpawn))
        (CallFunction|ChooseSecondSpawn)))))

(event Custom|ItemSpawned
  ;[1 1 1] Update Number of item already spawned
  (Math|Integer|DecrementInt (Variables|/Game/Core/GM_Lumiere.GM_Lumiere_C|GetNumberOfItems (.AsGM%20Lumiere (Utilities|Casting|CastToGM_Lumiere (Game|GetGameMode))))))

(event EventBeginPlay
  ;[1 1 1] Begin Play
  (Variables|Ref|SetGmLumiereRef (.AsGM%20Lumiere (Utilities|Casting|CastToGM_Lumiere (Game|GetGameMode))))
  (Components|StaticMesh|SetStaticMesh (Variables|Default|GetStaticMesh) 0)
  (Utilities|FlowControl|DelayUntilNextTick)
  (if (> (Variables|/Game/Core/GM_Lumiere.GM_Lumiere_C|GetNumberOfItems (Variables|Ref|GetGmLumiereRef)) 0)
    ;;[0.2417 0.53 1] Check Item is null
    (if (Utilities|Enum|Equal(Enum) (.Name (Utilities|Struct|BreakS_ItemData (Variables|Item|GetItem))) "Null")
      (CallFunction|SpawnFirstRandomItem)
      (CallFunction|ChooseSecondSpawn))))

(fn ConstructionScript)

(fn SpawnFirstRandomItem
  (bind _returnvalue (Game|GetGameMode))
  (bind _asgm_lumiere (Utilities|Casting|CastToGM_Lumiere _returnvalue))
  (bind _itemscanspawn (Variables|/Game/Core/GM_Lumiere.GM_Lumiere_C|GetItemsCanSpawn _asgm_lumiere))
  (bind _output_get (Variables|Item|SetItem (.OutItem (Utilities|Array|Random _itemscanspawn))))
  (Utilities|Array|RemoveItem _itemscanspawn _output_get)
  (CallFunction|ItemSpawned)
  (Components|StaticMesh|SetStaticMesh (Variables|Default|GetStaticMesh) (.Mesh (Utilities|Struct|BreakS_ItemData (Variables|Item|GetItem)))))

(fn SpawnSecondSetItem
  (bind _array_element (Utilities|Array|ForEachLoopwithBreak (Variables|/Game/Core/GM_Lumiere.GM_Lumiere_C|GetItemsCanSpawn (Variables|Ref|GetGmLumiereRef)) :!label _label)
    (:LoopBody
      (LocalVariables|SetSecondItem _array_element)
      (if (Utilities|Enum|Equal(Enum) (.SetType (Utilities|Struct|BreakS_ItemData (Variables|Item|GetItem))) (.SetType (Utilities|Struct|BreakS_ItemData (LocalVariables|GetSecondItem))))
        ;[0.2192 0.4144 1] Set Second Item
        (bind _output_get (Variables|BP_Item_C|SetItem (Variables|Spawns|GetSecondSetSpawn) (LocalVariables|GetSecondItem)))
        (Components|StaticMesh|SetStaticMesh (Variables|BP_Item_C|GetStaticMesh (Variables|Spawns|GetSecondSetSpawn)) (.Mesh (Utilities|Struct|BreakS_ItemData _output_get)))
        (Utilities|Array|RemoveItem (Variables|/Game/Core/GM_Lumiere.GM_Lumiere_C|GetItemsCanSpawn (Variables|Ref|GetGmLumiereRef)) (LocalVariables|GetSecondItem))
        (CallFunction|ItemSpawned)
        (goto _label Break)))))