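; Ice water pool hazard for two players that freezes a character entering its box, then respawns them from the sky.
; Overlap disables that player's input, gravity and velocity, then teleports them to the RespawnManager's top point on the left or right side.
; After a freeze timer, a per-player timeline lerps them toward the bottom point, then restores control.
; Player 2's fall lerps from Player 1's location and uses Play instead of PlayFromStart.
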(event OnComponentBeginOverlap(Box)
  (params (OverlappedComponent :type Primitive%20Component%20Object%20Reference) (OtherActor :type Actor%20Object%20Reference) (OtherComp :type Primitive%20Component%20Object%20Reference) (OtherBodyIndex :type Integer) (bFromSweep :type Boolean) (SweepResult :type Hit%20Result%20Structure%20%28by%20ref%29))
  (bind _asbp_character (Utilities|Casting|CastToBP_Character OtherActor))
  (switch int (Variables|/Game/Core/BP_Character.BP_Character_C|GetPlayerIndex _asbp_character)
    (:Default
      ;[0 0 0] Freeze then Respawn P2
      (if (not (Variables|/Game/Core/BP_Character.BP_Character_C|GetJustFell (Variables|Ref|GetPlayer2Ref))) :!label _label
        (Variables|/Game/Core/BP_Character.BP_Character_C|SetJustFell (Variables|Ref|GetPlayer2Ref) true)
        (CallFunction|StopPlayer (Variables|Ref|GetPlayer2Ref))
        (CallFunction|TeleportPlayer (Variables|Ref|GetPlayer2Ref))
        (Utilities|Time|SetTimerbyEvent (delegate Custom|Respawn%20Player%202) (Variables|Qualities|GetFreezeTime))))
    (:0
      ;[0 0 0] Freeze then Respawn P1
      (if (not (Variables|/Game/Core/BP_Character.BP_Character_C|GetJustFell (Variables|Ref|GetPlayer1Ref)))
        (Variables|/Game/Core/BP_Character.BP_Character_C|SetJustFell (Variables|Ref|GetPlayer1Ref) true)
        (CallFunction|StopPlayer (Variables|Ref|GetPlayer1Ref))
        (CallFunction|TeleportPlayer (Variables|Ref|GetPlayer1Ref))
        (Utilities|Time|SetTimerbyEvent (delegate Custom|Respawn%20Player%201) (Variables|Qualities|GetFreezeTime))))
    (:1
      (goto _label))))

(event Custom|Respawn%20Player%202
  (bind _respawnmanager (Variables|Qualities|GetRespawnManager))
  (bind _leftrespawnbottom (Variables|/Game/Blueprints/GPEs/BP_IceChunkManager.BP_IceChunkManager_C|GetLeftRespawnBottom _respawnmanager))
  ;[0 0 0] Freeze then Respawn P2
  (bind _fall (Timeline|Player%202%20falls%20from%20sky Play)
    (:Update
      (Transformation|SetActorLocationAndRotation (Variables|Ref|GetPlayer2Ref) (Math|Vector|Lerp(Vector) (Transformation|GetActorLocation (Variables|Ref|GetPlayer1Ref)) (Math|Vector|SelectVector (Transformation|GetWorldLocation (Variables|/Game/Blueprints/GPEs/BP_IceChunkManager.BP_IceChunkManager_C|GetRightRespawnBottom (Variables|Qualities|GetRespawnManager))) (Transformation|GetWorldLocation _leftrespawnbottom) (Variables|Qualities|GetRightSide)) _fall) (Transformation|GetWorldRotation _leftrespawnbottom) false true))
    (:Finished
      (CallFunction|UnfreezePlayer (Variables|Ref|GetPlayer2Ref)))))

(event Custom|Respawn%20Player%201
  (bind _respawnmanager (Variables|Qualities|GetRespawnManager))
  (bind _leftrespawnbottom (Variables|/Game/Blueprints/GPEs/BP_IceChunkManager.BP_IceChunkManager_C|GetLeftRespawnBottom _respawnmanager))
  ;[0 0 0] Freeze then Respawn P1
  (Variables|Ref|SetOriginal%20Player%20Scale (Transformation|GetWorldScale (Variables|/Game/Core/BP_Character.BP_Character_C|GetCylinder (Variables|Ref|GetPlayer1Ref))))
  (Variables|Default|SetOriginal%20Player%20Rotation (Transformation|GetWorldRotation (Variables|/Game/Core/BP_Character.BP_Character_C|GetCylinder (Variables|Ref|GetPlayer1Ref))))
  (bind _fall (Timeline|Player%201%20falls%20from%20sky PlayFromStart)
    (:Update
      (Transformation|SetActorLocationAndRotation (Variables|Ref|GetPlayer1Ref) (Math|Vector|Lerp(Vector) (Transformation|GetActorLocation (Variables|Ref|GetPlayer1Ref)) (Math|Vector|SelectVector (Transformation|GetWorldLocation (Variables|/Game/Blueprints/GPEs/BP_IceChunkManager.BP_IceChunkManager_C|GetRightRespawnBottom (Variables|Qualities|GetRespawnManager))) (Transformation|GetWorldLocation _leftrespawnbottom) (Variables|Qualities|GetRightSide)) _fall) (Transformation|GetWorldRotation _leftrespawnbottom) false true))
    (:Finished
      (CallFunction|UnfreezePlayer (Variables|Ref|GetPlayer1Ref)))))

(event EventBeginPlay
  (Utilities|FlowControl|DelayUntilNextTick)
  (bind _asbp_character (Utilities|Casting|CastToBP_Character (Game|GetPlayerCharacter 0)))
  (Variables|Ref|SetPlayer1Ref _asbp_character)
  (bind _asbp_character_2 (Utilities|Casting|CastToBP_Character (Game|GetPlayerCharacter 1)))
  (Variables|Ref|SetPlayer2Ref _asbp_character_2))

(fn ConstructionScript)

(fn StopPlayer
  (params (Player :type BP%20Character%20Object%20Reference))
  (bind _playerindex (Variables|/Game/Core/BP_Character.BP_Character_C|GetPlayerIndex Player))
  (bind _returnvalue (Game|GetPlayerController _playerindex))
  (Input|RemoveMappingContext _returnvalue "/Game/Input/IMC_MainContols.IMC_MainContols" "(bIgnoreAllPressedKeysUntilRelease=True,bForceImmediately=False,bNotifyUserSettings=False)")
  (Input|DisableInput (Game|GetPlayerCharacter _playerindex) _returnvalue)
  (Variables|/Script/Engine.CharacterMovementComponent|SetGravityScale (Variables|/Script/Engine.Character|GetCharacterMovement Player) 0.0)
  (Variables|/Script/Engine.MovementComponent|SetVelocity (Variables|/Script/Engine.Character|GetCharacterMovement Player) "0, 0, 0"))

(fn TeleportPlayer
  (params (Player :type Actor%20Object%20Reference))
  (Transformation|SetActorLocationAndRotation Player (Math|Vector|SelectVector (Transformation|GetWorldLocation (Variables|/Game/Blueprints/GPEs/BP_IceChunkManager.BP_IceChunkManager_C|GetRightRespawnTop (Variables|Qualities|GetRespawnManager))) (Transformation|GetWorldLocation (Variables|/Game/Blueprints/GPEs/BP_IceChunkManager.BP_IceChunkManager_C|GetLeftRespawnTop (Variables|Qualities|GetRespawnManager))) (Variables|Qualities|GetRightSide)) "0, 0, 0" false true))

(fn UnfreezePlayer
  (params (Player :type BP%20Character%20Object%20Reference))
  (bind _playerindex (Variables|/Game/Core/BP_Character.BP_Character_C|GetPlayerIndex Player))
  (Variables|/Game/Core/BP_Character.BP_Character_C|SetJustFell Player false)
  (Variables|/Script/Engine.CharacterMovementComponent|SetGravityScale (Variables|/Script/Engine.Character|GetCharacterMovement Player) 1.0)
  (Input|EnableInput (Game|GetPlayerCharacter _playerindex) (Game|GetPlayerController _playerindex)))