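; Ice water pool hazard for two players that freezes a fallen character and respawns it on the side it fell in from.
; Left and right sensors lock in each player's entry side until respawn completes.
; The center box disables input, gravity and velocity, then teleports the player to the RespawnManager's matching point.
; After a freeze timer, a timeline lerps the player to that side's respawn point before restoring control.
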(event OnComponentBeginOverlap(Box)
  (params (OverlappedComponent :type Primitive%20Component%20Object%20Reference) (OtherActor :type Actor%20Object%20Reference) (OtherComp :type Primitive%20Component%20Object%20Reference) (OtherBodyIndex :type Integer) (bFromSweep :type Boolean) (SweepResult :type Hit%20Result%20Structure%20%28by%20ref%29))
  (bind _asbp_character (Utilities|Casting|CastToBP_Character OtherActor))
  (switch int (Variables|/Game/Core/BP_Character.BP_Character_C|GetPlayerIndex _asbp_character)
    (:0
      ;[0 0 0] Freeze then Respawn P1
      (if (not (Variables|/Game/Core/BP_Character.BP_Character_C|GetJustFell (Variables|Ref|GetPlayer1Ref)))
        (Variables|/Game/Core/BP_Character.BP_Character_C|SetJustFell (Variables|Ref|GetPlayer1Ref) true)
        (CallFunction|StopPlayer (Variables|Ref|GetPlayer1Ref))
        (CallFunction|TeleportPlayer1 (Variables|Ref|GetPlayer1Ref))
        (Utilities|Time|SetTimerbyEvent (delegate Custom|Respawn%20Player%201) (Variables|Qualities|GetFreezeTime))))
    (:1
      ;[0 0 0] Freeze then Respawn P2
      (if (not (Variables|/Game/Core/BP_Character.BP_Character_C|GetJustFell (Variables|Ref|GetPlayer2Ref)))
        (Variables|/Game/Core/BP_Character.BP_Character_C|SetJustFell (Variables|Ref|GetPlayer2Ref) true)
        (CallFunction|StopPlayer (Variables|Ref|GetPlayer2Ref))
        (CallFunction|TeleportPlayer2 (Variables|Ref|GetPlayer2Ref))
        (Utilities|Time|SetTimerbyEvent (delegate Custom|Respawn%20Player%202) (Variables|Qualities|GetFreezeTime))))))

(event OnComponentBeginOverlap(LeftSensor)
  (params (OverlappedComponent :type Primitive%20Component%20Object%20Reference) (OtherActor :type Actor%20Object%20Reference) (OtherComp :type Primitive%20Component%20Object%20Reference) (OtherBodyIndex :type Integer) (bFromSweep :type Boolean) (SweepResult :type Hit%20Result%20Structure%20%28by%20ref%29))
  ;[0 0 0] Check which side the player fell in from
  (bind _asbp_character (Utilities|Casting|CastToBP_Character OtherActor))
  (switch int (Variables|/Game/Core/BP_Character.BP_Character_C|GetPlayerIndex _asbp_character)
    (:0
      (if (not (Variables|Default|GetPlayer1LockedIn))
        (Variables|Default|SetPlayer1LockedIn true)
        (Variables|Default|SetPlayer1RightSide false)))
    (:1
      (if (not (Variables|Default|GetPlayer2LockedIn))
        (Variables|Default|SetPlayer2LockedIn true)
        (Variables|Default|SetPlayer2RightSide false)))))

(event OnComponentBeginOverlap(RightSensor)
  (params (OverlappedComponent :type Primitive%20Component%20Object%20Reference) (OtherActor :type Actor%20Object%20Reference) (OtherComp :type Primitive%20Component%20Object%20Reference) (OtherBodyIndex :type Integer) (bFromSweep :type Boolean) (SweepResult :type Hit%20Result%20Structure%20%28by%20ref%29))
  ;[0 0 0] Check which side the player fell in from
  (bind _asbp_character (Utilities|Casting|CastToBP_Character OtherActor))
  (switch int (Variables|/Game/Core/BP_Character.BP_Character_C|GetPlayerIndex _asbp_character)
    (:0
      (if (not (Variables|Default|GetPlayer1LockedIn))
        (Variables|Default|SetPlayer1LockedIn true)
        (Variables|Default|SetPlayer1RightSide true)))
    (:1
      (if (not (Variables|Default|GetPlayer2LockedIn))
        (Variables|Default|SetPlayer2LockedIn true)
        (Variables|Default|SetPlayer2RightSide true)))))

(event Custom|Respawn%20Player%202
  (bind _respawnpointleft (Variables|Qualities|GetRespawnPointLeft))
  (bind _respawnpointright (Variables|Qualities|GetRespawnPointRight))
  (bind _player2rightside (Variables|Default|GetPlayer2RightSide))
  (bind _returnvalue (select _player2rightside _respawnpointright _respawnpointleft))
  ;[0 0 0] Freeze then Respawn P2
  (bind _fall (Timeline|Player%202%20falls%20from%20sky Play)
    (:Update
      (Transformation|SetActorLocationAndRotation (Variables|Ref|GetPlayer2Ref) (Math|Vector|Lerp(Vector) (Transformation|GetActorLocation (Variables|Ref|GetPlayer2Ref)) (Transformation|GetActorLocation _returnvalue) _fall) (Transformation|GetActorRotation _returnvalue) false true))
    (:Finished
      (Utilities|FlowControl|Delay 1.0)
      (CallFunction|UnfreezePlayer2 (Variables|Ref|GetPlayer2Ref)))))

(event Custom|Respawn%20Player%201
  (bind _respawnpointright (Variables|Qualities|GetRespawnPointRight))
  (bind _player1rightside (Variables|Default|GetPlayer1RightSide))
  (bind _respawnpointleft (Variables|Qualities|GetRespawnPointLeft))
  (bind _returnvalue (select _player1rightside _respawnpointright _respawnpointleft))
  ;[0 0 0] Freeze then Respawn P1
  (bind _fall (Timeline|Player%201%20falls%20from%20sky PlayFromStart)
    (:Update
      (Transformation|SetActorLocationAndRotation (Variables|Ref|GetPlayer1Ref) (Math|Vector|Lerp(Vector) (Transformation|GetActorLocation (Variables|Ref|GetPlayer1Ref)) (Transformation|GetActorLocation _returnvalue) _fall) (Transformation|GetActorRotation _returnvalue) false true))
    (:Finished
      (Utilities|FlowControl|Delay 1.0)
      (CallFunction|UnfreezePlayer1 (Variables|Ref|GetPlayer1Ref)))))

(event EventBeginPlay
  (bind _asbp_character (Utilities|Casting|CastToBP_Character (Game|GetPlayerCharacter 0)))
  (Variables|Ref|SetPlayer1Ref _asbp_character)
  (bind _asbp_character_2 (Utilities|Casting|CastToBP_Character (Game|GetPlayerCharacter 1)))
  (Variables|Ref|SetPlayer2Ref _asbp_character_2))

(fn ConstructionScript)

(fn StopPlayer
  (params (Player :type BP%20Character%20Object%20Reference))
  (bind _playerindex (Variables|/Game/Core/BP_Character.BP_Character_C|GetPlayerIndex Player))
  (Input|DisableInput (Game|GetPlayerCharacter _playerindex) (Game|GetPlayerController _playerindex))
  (Variables|/Script/Engine.CharacterMovementComponent|SetGravityScale (Variables|/Script/Engine.Character|GetCharacterMovement Player) 0.0)
  (Variables|/Script/Engine.MovementComponent|SetVelocity (Variables|/Script/Engine.Character|GetCharacterMovement Player) "0, 0, 0"))

(fn TeleportPlayer1
  (params (Player :type Actor%20Object%20Reference))
  (Transformation|SetActorLocationAndRotation Player (Math|Vector|SelectVector (Transformation|GetWorldLocation (Variables|/Game/Blueprints/GPEs/BP_IceChunkManager.BP_IceChunkManager_C|GetRightRespawn (Variables|Qualities|GetRespawnManager))) (Transformation|GetWorldLocation (Variables|/Game/Blueprints/GPEs/BP_IceChunkManager.BP_IceChunkManager_C|GetLeftRespawn (Variables|Qualities|GetRespawnManager))) (Variables|Default|GetPlayer1RightSide)) "0, 0, 0" false true))

(fn UnfreezePlayer1
  (params (Player :type BP%20Character%20Object%20Reference))
  (bind _playerindex (Variables|/Game/Core/BP_Character.BP_Character_C|GetPlayerIndex Player))
  (Variables|/Game/Core/BP_Character.BP_Character_C|SetJustFell Player false)
  (Variables|Default|SetPlayer1LockedIn false)
  (Variables|/Script/Engine.CharacterMovementComponent|SetGravityScale (Variables|/Script/Engine.Character|GetCharacterMovement Player) 1.0)
  (Input|EnableInput (Game|GetPlayerCharacter _playerindex) (Game|GetPlayerController _playerindex)))

(fn TeleportPlayer2
  (params (Player :type Actor%20Object%20Reference))
  (Transformation|SetActorLocationAndRotation Player (Math|Vector|SelectVector (Transformation|GetWorldLocation (Variables|/Game/Blueprints/GPEs/BP_IceChunkManager.BP_IceChunkManager_C|GetRightRespawn (Variables|Qualities|GetRespawnManager))) (Transformation|GetWorldLocation (Variables|/Game/Blueprints/GPEs/BP_IceChunkManager.BP_IceChunkManager_C|GetLeftRespawn (Variables|Qualities|GetRespawnManager))) (Variables|Default|GetPlayer2RightSide)) "0, 0, 0" false true))

(fn UnfreezePlayer2
  (params (Player :type BP%20Character%20Object%20Reference))
  (bind _playerindex (Variables|/Game/Core/BP_Character.BP_Character_C|GetPlayerIndex Player))
  (Variables|/Game/Core/BP_Character.BP_Character_C|SetJustFell Player false)
  (Variables|Default|SetPlayer2LockedIn false)
  (Variables|/Script/Engine.CharacterMovementComponent|SetGravityScale (Variables|/Script/Engine.Character|GetCharacterMovement Player) 1.0)
  (Input|EnableInput (Game|GetPlayerCharacter _playerindex) (Game|GetPlayerController _playerindex)))