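; BP_BumpBush is a bush obstacle that launches the player character on overlap, with sound and Niagara feedback.
; Launch velocity comes from BushBumpForceAndNormal, whose visible direction and clamped-speed math appears unconnected.
; A timeline scales the mesh and raises the glow on a swapped emissive dynamic material.
; The trigger sphere shrinks to zero radius during the animation to block retriggers, then radius, scale and material are restored.
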(event OnComponentBeginOverlap(Sphere)
  (params (OverlappedComponent :type Primitive%20Component%20Object%20Reference) (OtherActor :type Actor%20Object%20Reference) (OtherComp :type Primitive%20Component%20Object%20Reference) (OtherBodyIndex :type Integer) (bFromSweep :type Boolean) (SweepResult :type Hit%20Result%20Structure%20%28by%20ref%29))
  (bind _emissivebushmaterial (Variables|Default|GetEmissiveBushMaterial))
  (bind _vfxfeedback (Variables|Default|GetVFXFeedback))
  ;[1 1 1] Checking for player
  (bind _asbp_character (Utilities|Casting|CastToBP_Character OtherActor))
  ;[1 1 1] Bouncing player back
  (Character|LaunchCharacter _asbp_character (Utilities|BushBumpForceandNormal _asbp_character) true true)
  ;[1 1 1] Play sound and FX
  (Audio|PlaySound2D (Variables|/Game/Blueprints/PDA/PDA_SFXList.PDA_SFXList_C|GetBounceSounds (Variables|Default|GetSFX_DARef)) 1.0 1.0 0.0 0 0)
  (Transformation|SetWorldRotation _vfxfeedback (Math|Rotator|MakeRotator 0.0 0.0 (.yaw (Math|Rotator|MakeRotfromX (* (.Normal (Collision|BreakHitResult SweepResult)) -1.0)))) false false)
  ;;[1 0.5034 0.1009] Play fx
  (Components|Activation|Activate _vfxfeedback false)
  ;[1 1 1] Making the mesh bounce
  (Components|Sphere|SetSphereRadius (Variables|Default|GetSphere) 0.0 true)
  (Rendering|Material|SetMaterial (Variables|Default|GetMesh) 0 (Variables|Default|GetEmissiveBushMaterial))
  (bind _newtrack_0 (Timeline|Feedback PlayFromStart)
    (:Update
      (Transformation|SetRelativeScale3D (Variables|Default|GetMesh) (* (Variables|BounceVariables|GetBumpScaleUp) _newtrack_0))
      ;;[1 0.6856 0.2516] Make the mesh glow
      (bind _returnvalue (Rendering|Material|GetScalarParameterValue _emissivebushmaterial "EmissivePower" :!class /Script/Engine.MaterialInstanceDynamic))
      (Rendering|Material|SetScalarParameterValue _emissivebushmaterial "EmissivePower" (Math|Float|Lerp _returnvalue (Variables|MaterialOnBounce|GetEmissivePower) _newtrack_0) :!class /Script/Engine.MaterialInstanceDynamic))
    (:Finished
      (Components|Sphere|SetSphereRadius (Variables|Default|GetSphere) (Variables|BounceVariables|GetCollisionRadius) true)
      (Transformation|SetRelativeScale3D (Variables|Default|GetMesh) "1.000000,1.000000,1.000000")
      (Rendering|Material|SetMaterial (Variables|Default|GetMesh) 0 (Variables|Default|GetBaseMaterial))
      (Components|Activation|Deactivate (Variables|Default|GetVFXFeedback)))))

(event EventBeginPlay
  ;[1 1 1] Begin Play
  (Class|NiagaraComponent|SetAsset (Variables|Default|GetVFXFeedback) (Variables|VFX|GetBushVFX) true)
  ;;[0.4158 0.6112 1] SetMaterials
  (bind _returnvalue (Rendering|Material|CreateDynamicMaterialInstance (Rendering|Material|GetMaterial (Variables|Default|GetMesh) 0) "None" "None" :!class /Script/Engine.KismetMaterialLibrary))
  (Variables|Default|SetBaseMaterial _returnvalue)
  (bind _returnvalue_2 (Rendering|Material|CreateDynamicMaterialInstance (Variables|MaterialOnBounce|GetEmissiveMaterial) "None" "None" :!class /Script/Engine.KismetMaterialLibrary))
  (bind _output_get (Variables|Default|SetEmissiveBushMaterial _returnvalue_2))
  (bind _returnvalue_3 (Rendering|Material|GetScalarParameterValue _output_get "EmissivePower" :!class /Script/Engine.MaterialInstanceDynamic))
  (Variables|MaterialOnBounce|SetEmissivePower _returnvalue_3)
  (Rendering|Material|SetScalarParameterValue _output_get "EmissivePower" 0.0 :!class /Script/Engine.MaterialInstanceDynamic))

(fn ConstructionScript
  (Components|StaticMesh|SetStaticMesh (Variables|Default|GetMesh) (Variables|Mesh|GetBushMesh))
  (Components|Sphere|SetSphereRadius (Variables|Default|GetSphere) (Variables|BounceVariables|GetCollisionRadius) true))