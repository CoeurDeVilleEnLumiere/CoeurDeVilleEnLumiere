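; BP_DiscoTile is a floor tile that lights up in a player-specific material when Player 1 or Player 2 steps on it.
; Player references are cached when GM_Lumiere signals game start, then compared against actors overlapping the Box.
; On exit, the FadeLight timeline lerps the dynamic material's "Strenght" parameter to zero, then restores the base material.
; The construction script exposes the tile mesh and collision box transform and size.
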(event OnComponentBeginOverlap(Box)
  (params (OverlappedComponent :type Primitive%20Component%20Object%20Reference) (OtherActor :type Actor%20Object%20Reference) (OtherComp :type Primitive%20Component%20Object%20Reference) (OtherBodyIndex :type Integer) (bFromSweep :type Boolean) (SweepResult :type Hit%20Result%20Structure%20%28by%20ref%29))
  ;[1 1 1] Check if P1 or P2 are walking on a tile and light it up
  (if (== OtherActor (Variables|Default|GetPlayer1Ref))
    (bind _returnvalue (Rendering|Material|CreateDynamicMaterialInstance (Variables|TileVariables|GetPlayer1Material) "None" "None" :!class /Script/Engine.KismetMaterialLibrary))
    (bind _output_get (Variables|Default|SetCurrentMaterial _returnvalue))
    (Rendering|Material|SetMaterial (Variables|Default|GetTile) 0 _output_get)
    (elif (== OtherActor (Variables|Default|GetPlayer2Ref))
      (bind _returnvalue_2 (Rendering|Material|CreateDynamicMaterialInstance (Variables|TileVariables|GetPlayer2Material) "None" "None" :!class /Script/Engine.KismetMaterialLibrary))
      (bind _output_get_2 (Variables|Default|SetCurrentMaterial _returnvalue_2))
      (Rendering|Material|SetMaterial (Variables|Default|GetTile) 0 _output_get_2))))

(event OnComponentEndOverlap(Box)
  (params (OverlappedComponent :type Primitive%20Component%20Object%20Reference) (OtherActor :type Actor%20Object%20Reference) (OtherComp :type Primitive%20Component%20Object%20Reference) (OtherBodyIndex :type Integer))
  (bind _currentmaterial (Variables|Default|GetCurrentMaterial))
  ;[1 1 1] Fade Light when player leave the tile
  (if (or (== OtherActor (Variables|Default|GetPlayer1Ref)) (== OtherActor (Variables|Default|GetPlayer2Ref)))
    (bind _alpha (Timeline|FadeLight PlayFromStart)
      (:Update
        (bind _returnvalue (Rendering|Material|GetScalarParameterValue _currentmaterial "Strenght" :!class /Script/Engine.MaterialInstanceDynamic))
        (Rendering|Material|SetScalarParameterValue _currentmaterial "Strenght" (Math|Float|Lerp _returnvalue 0.0 _alpha) :!class /Script/Engine.MaterialInstanceDynamic))
      (:Finished
        (Rendering|Material|SetMaterial (Variables|Default|GetTile) 0 (Variables|Default|GetBaseMaterial))))))

(event Custom|GameStart_Event
  ;[1 1 1] Set P1 and P2 variable at game start
  (bind _asbp_character (Utilities|Casting|CastToBP_Character (Game|GetPlayerCharacter 0)))
  (Variables|Default|SetPlayer1Ref _asbp_character)
  (bind _asbp_character_2 (Utilities|Casting|CastToBP_Character (Game|GetPlayerCharacter 1)))
  (Variables|Default|SetPlayer2Ref _asbp_character_2))

(event EventBeginPlay
  ;[1 1 1] Begin Play
  (bind _returnvalue (Rendering|Material|CreateDynamicMaterialInstance (Rendering|Material|GetMaterial (Variables|Default|GetTile) 0) "None" "None" :!class /Script/Engine.KismetMaterialLibrary))
  (Variables|Default|SetBaseMaterial _returnvalue)
  (EventDispatchers|AssignGameStart (.AsGM%20Lumiere (Utilities|Casting|CastToGM_Lumiere (Game|GetGameMode))) (delegate Custom|GameStart_Event)))

(fn ConstructionScript
  (bind _box (Variables|Default|GetBox))
  (Components|StaticMesh|SetStaticMesh (Variables|Default|GetTile) (Variables|TileVariables|GetTileMesh))
  (Transformation|SetRelativeLocation _box (Variables|CollisionVariables|GetCollisionBoxLocation) false false)
  (Transformation|SetRelativeRotation _box (Variables|CollisionVariables|GetCollisionBoxRotation) false false)
  (Components|Box|SetBoxExtent _box (Variables|CollisionVariables|GetCollisionBoxSize) true))