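; Bouncing gameplay element that knocks BP_Character backward when it hits the collision sphere.
; The hit launches the character opposite its capsule's forward vector, scaled by BounceForce, and plays a 2D bounce sound from SFXDARef.
; BeginPlay creates base and active-bush dynamic materials and caches glow strength, but never applies them.
; The bush glow and fade timelines are never triggered, and InvalidateFadeTimer is empty.
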(event OnComponentHit(CollisionSphere)
  (params (HitComponent :type Primitive%20Component%20Object%20Reference) (OtherActor :type Actor%20Object%20Reference) (OtherComp :type Primitive%20Component%20Object%20Reference) (NormalImpulse :type Vector :default "0, 0, 0") (Hit :type Hit%20Result%20Structure%20%28by%20ref%29))
  (bind _asbp_character (Utilities|Casting|CastToBP_Character OtherActor))
  (Character|LaunchCharacter _asbp_character (* (Math|Vector|GetForwardVector (Transformation|GetWorldRotation (Variables|/Script/Engine.Character|GetCapsuleComponent _asbp_character))) -1.0 (Variables|Default|GetBounceForce)) false false)
  (Audio|PlaySound2D (Variables|/Game/Blueprints/PDA/PDA_SFXList.PDA_SFXList_C|GetBounceSounds (Variables|Default|GetSFX_DARef)) 1.0 1.0 0.0 0 0))

(event Custom|InvalidateFadeTimer)

(event EventBeginPlay
  (bind _returnvalue (Rendering|Material|CreateDynamicMaterialInstance (Rendering|Material|GetMaterial (Variables|Default|GetSphere) 0) "None" "None" :!class /Script/Engine.KismetMaterialLibrary))
  (Variables|Default|SetBaseMaterial _returnvalue)
  (bind _returnvalue_2 (Rendering|Material|CreateDynamicMaterialInstance "/Game/Art/Materials/Instances/MI_ActiveBush.MI_ActiveBush" "None" "None" :!class /Script/Engine.KismetMaterialLibrary))
  (bind _output_get (Variables|Default|SetCurrentBushMaterial _returnvalue_2))
  (bind _returnvalue_3 (Rendering|Material|GetScalarParameterValue _output_get "EmissivePower" :!class /Script/Engine.MaterialInstanceDynamic))
  (Variables|Default|SetGlowStrength _returnvalue_3))

(fn ConstructionScript)