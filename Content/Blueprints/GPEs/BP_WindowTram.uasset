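; BP_WindowTram is an actor that spawns a BP_TramLight at the start of its spline on BeginPlay and is meant to move it along that path.
; MovingTram loops over spline point indices, restarting a Timeline that lerps location between neighbouring points with sweep.
; The loop does not wait for the Timeline, so updates see only the final index.
; Rotation interpolation nodes are left unconnected.
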(event Custom|MovingTram
  (params (Target :type Actor%20Object%20Reference))
  (for _index (range 1 (Spline|GetNumberOfSplinePoints (Variables|Default|GetSpline)))
    (bind _alpha (Timeline|Timeline PlayFromStart)
      (:Update
        (Transformation|SetActorLocationAndRotation Target (Math|Vector|Lerp(Vector) (Spline|GetLocationatSplinePoint (Variables|Default|GetSpline) (- _index 1) "World") (Spline|GetLocationatSplinePoint (Variables|Default|GetSpline) _index "World") _alpha) "0, 0, 0" true)))))

(event EventBeginPlay
  (bind _returnvalue (Game|SpawnActorfromClass "/Game/Maps/Mathias_LevelBlocking/Blueprints/BP_TramLight.BP_TramLight_C" (Math|Conversions|ToTransform(Vector) (Spline|GetLocationatSplinePoint (Variables|Default|GetSpline) 0 "World")) "Undefined" "MultiplyWithRoot" 0 0))
  (CallFunction|MovingTram _returnvalue))

(fn ConstructionScript)