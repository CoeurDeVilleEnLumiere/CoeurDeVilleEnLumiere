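; BP_TramLight is a tram signal whose two lights, LightA and LightB, blink alternately.
; Activation sets StayOn, then chained one-shot timers swap the on and off materials between the meshes after each Delay.
; At the end of each cycle, StayOn decides whether blinking restarts or both lights switch off.
; Nothing in this graph clears StayOn.
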(event Custom|ActivateLight_Event
  ;[1 1 1] Blink Between 2 Lights
  (Variables|Default|SetStayOn true)
  (Rendering|Material|SetMaterial (Variables|Default|GetLightA) 0 (Variables|Default|GetOnMaterial))
  (Rendering|Material|SetMaterial (Variables|Default|GetLightB) 0 (Variables|Default|GetOffMaterial))
  (Utilities|Time|SetTimerbyEvent (delegate Custom|SwitchLight) (Variables|Default|GetDelay)))

(event Custom|ExitOrRestart
  ;[1 1 1] Check if Tram is still passing
  (if (Variables|Default|GetStayOn)
    (CallFunction|ActivateLightEvent)
    (else
      (CallFunction|TurnOffLights))))

(event Custom|SwitchLight
  ;[1 1 1] Blink Between 2 Lights
  (Rendering|Material|SetMaterial (Variables|Default|GetLightB) 0 (Variables|Default|GetOnMaterial))
  (Rendering|Material|SetMaterial (Variables|Default|GetLightA) 0 (Variables|Default|GetOffMaterial))
  (Utilities|Time|SetTimerbyEvent (delegate Custom|ExitOrRestart) (Variables|Default|GetDelay)))

(event Custom|TurnOffLights
  ;[1 1 1] Turn Lights Off
  (Rendering|Material|SetMaterial (Variables|Default|GetLightA) 0 (Variables|Default|GetOffMaterial))
  (Rendering|Material|SetMaterial (Variables|Default|GetLightB) 0 (Variables|Default|GetOffMaterial)))

(fn ConstructionScript)