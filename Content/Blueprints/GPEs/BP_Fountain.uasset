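; BP_Fountain is a fountain obstacle that periodically pulses water and launches any BP_Character that begins overlapping its Sphere.
; A Cooldown timeline and PulseTimeline trigger each other in a loop, collapsing then scaling the Sphere and Cylinder.
; The launch adds horizontal velocity and zeroes vertical velocity; its look-at uses the fountain's location as both start and target, giving a fixed direction rather than radial knockback.
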(event OnComponentBeginOverlap(Sphere)
  (params (OverlappedComponent :type Primitive%20Component%20Object%20Reference) (OtherActor :type Actor%20Object%20Reference) (OtherComp :type Primitive%20Component%20Object%20Reference) (OtherBodyIndex :type Integer) (bFromSweep :type Boolean) (SweepResult :type Hit%20Result%20Structure%20%28by%20ref%29))
  (bind _returnvalue (Transformation|GetActorLocation))
  (bind _returnvalue_2 (Transformation|GetActorLocation))
  (bind _returnvalue_3 (Math|Rotator|FindLookatRotation _returnvalue_2 _returnvalue))
  ;[1 1 1] Launch Character on collision
  (bind _asbp_character (Utilities|Casting|CastToBP_Character OtherActor))
  (Character|LaunchCharacter _asbp_character (* (Math|Vector|GetForwardVector (Math|Rotator|MakeRotator (.roll _returnvalue_3) 0.0 (.yaw _returnvalue_3))) 1e+03) false true))

(event Custom|Pulse
  ;[1 1 1] Pulse Water
  (bind _newtrack_0 (Timeline|PulseTimeline PlayFromStart)
    (:Update
      (Transformation|SetRelativeScale3D (Variables|Default|GetSphere) (* "1.600000,1.600000,1.600000" _newtrack_0))
      (Transformation|SetRelativeScale3D (Variables|Default|GetCylinder) (Math|Vector|MakeVector _newtrack_0 _newtrack_0 0.1)))
    (:Finished
      (CallFunction|ResetPulse))))

(event Custom|ResetPulse
  ;[1 1 1] Begin Play / Reset
  (Transformation|SetRelativeScale3D (Variables|Default|GetSphere) "0, 0, 0")
  (Transformation|SetRelativeScale3D (Variables|Default|GetCylinder) "0, 0, 0")
  (Timeline|Cooldown PlayFromStart
    (:Finished
      (CallFunction|Pulse))))

(event EventBeginPlay
  ;[1 1 1] Begin Play / Reset
  (Components|Timeline|SetPlayRate (Variables|Default|GetCooldown) 0.2)
  (Transformation|SetRelativeScale3D (Variables|Default|GetSphere) "0, 0, 0")
  (Transformation|SetRelativeScale3D (Variables|Default|GetCylinder) "0, 0, 0")
  (Timeline|Cooldown PlayFromStart
    (:Finished
      (CallFunction|Pulse))))

(fn ConstructionScript)