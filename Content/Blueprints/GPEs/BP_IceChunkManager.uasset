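; Manages timed ice-breaking events in a match, temporarily sinking sets of ice chunks (center, mid, outer or all).
; A data asset (DARef) sets the order and timing of up to four events, chained through timers.
; Each set flashes a warning material, sinks via timeline with VFX, schedules the next event, then rises after a delay.
; An alternative random-chunk breaking path remains, but its starting timer is disconnected.
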(event Custom|Break%20Ice%20Chunk
  (Utilities|Time|InvalidateTimerHandle (stale Custom|IceBreakingSign _returnvalue))
  (for _array_element (Variables|Unused|GetIceChunksToDestroy)
    (Utilities|IsValid _array_element
      (:Is%20Valid
        (Transformation|SetActorLocation _array_element (Math|Vector|MakeVector (.x (Transformation|GetWorldLocation (Variables|/Script/Engine.StaticMeshActor|GetStaticMeshComponent _array_element))) (.y (Transformation|GetWorldLocation (Variables|/Script/Engine.StaticMeshActor|GetStaticMeshComponent _array_element))) (- (.z (Transformation|GetWorldLocation (Variables|/Script/Engine.StaticMeshActor|GetStaticMeshComponent _array_element))) 1e+03)) false false))))
  (if (not (Utilities|Array|IsEmpty (Variables|Chunks|GetAllIceChunks)))
    (Utilities|FlowControl|Delay (Variables|Unused|GetBreakIceInterval))
    (CallFunction|IceBreakingSign)))

(event Custom|IceBreakingSign
  (CallFunction|LightUpRandomIceChunk)
  (Utilities|FlowControl|DelayUntilNextTick)
  (CallFunction|LightUpRandomIceChunk)
  (Utilities|FlowControl|DelayUntilNextTick)
  (CallFunction|LightUpRandomIceChunk)
  (bind _returnvalue (Utilities|Time|SetTimerbyEvent (delegate Custom|Break%20Ice%20Chunk) (Variables|Unused|GetSignTime))))

(event Custom|Sink%20Chunk%20Set
  (params (ActiveChunksTo%20Sink :type Array%20of%20Static%20Mesh%20Actor%20Object%20References))
  ;[0 0 0] Sink breaking ice mesh set
  (for _array_element ActiveChunksTo%20Sink
    (Niagara|SpawnSystemAttached (Variables|VFX|GetIceSinkingVFX) (Variables|/Script/Engine.Actor|GetRootComponent _array_element) "None" "0, 0, 0" "90.000000,0.000000,0.000000" "SnapToTarget" false))
  (bind _sinkspeed (Timeline|SinkIceChunks PlayFromStart)
    (:Update
      (for _array_element_2 ActiveChunksTo%20Sink
        (Transformation|SetActorLocation _array_element_2 (Math|Vector|MakeVector (.X (Math|Vector|BreakVector (Transformation|GetActorLocation _array_element_2))) (.Y (Math|Vector|BreakVector (Transformation|GetActorLocation _array_element_2))) (Math|Float|Lerp (Variables|Default|GetOriginalZPosition) (Variables|Default|GetOffsetZPosition) _sinkspeed)) false false)))
    (:Finished
      (CallFunction|BreakSomeIce)
      (Utilities|FlowControl|Delay (Variables|/Game/Blueprints/PDA/PDA_IceChunkManager.PDA_IceChunkManager_C|GetSinkDuration (Variables|Core|GetDARef)))
      (CallFunction|BringBackIceChunks ActiveChunksTo%20Sink))))

(event Custom|Bring%20Back%20Ice%20Chunks
  (params (IceChunksToRaise :type Array%20of%20Static%20Mesh%20Actor%20Object%20References))
  ;[0 0 0] Raise breaking ice mesh set
  (bind _raisespeed (Timeline|RaiseIceChunks PlayFromStart)
    (:Update
      (for _array_element IceChunksToRaise
        (Transformation|SetActorLocation _array_element (Math|Vector|MakeVector (.x (Transformation|GetActorLocation _array_element)) (.y (Transformation|GetActorLocation _array_element)) (Math|Float|Lerp (Variables|Default|GetOffsetZPosition) (Variables|Default|GetOriginalZPosition) _raisespeed)) false false)))))

(event Custom|Qeue%20Ice%20Chunk%20Set
  (params (Active%20Chunk%20Set :type Array%20of%20Static%20Mesh%20Actor%20Object%20References))
  ;[0 0 0] Breaking Ice Sign
  (for _array_element Active%20Chunk%20Set
    (bind _output_get (Variables|Core|SetActiveChunk _array_element))
    (Rendering|Material|SetMaterial (Variables|/Script/Engine.StaticMeshActor|GetStaticMeshComponent _output_get) 0 (Variables|Core|GetBreakingSignMaterial)))
  (Utilities|Time|SetTimerbyEvent (delegate Custom|Sink%20Side%20Chunks) (Variables|/Game/Blueprints/PDA/PDA_IceChunkManager.PDA_IceChunkManager_C|GetSignTime (Variables|Core|GetDARef))))

(event Custom|Break%20Edges
  ;[0 0 0] Separate events for separate ice sets
  (CallFunction|QeueIceChunkSet (Variables|Chunks|GetOuterIceChunks)))

(event Custom|Sink%20Side%20Chunks
  ;[0 0 0] Breaking Ice Sign
  (for _array_element (stale Custom|Qeue%20Ice%20Chunk%20Set Active%20Chunk%20Set)
    (Utilities|IsValid _array_element
      (:Is%20Valid
        (Rendering|Material|SetMaterial (Variables|/Script/Engine.StaticMeshActor|GetStaticMeshComponent _array_element) 0 (Variables|Core|GetOriginal%20Material))
        (Variables|Default|SetOriginalZPosition (.z (Transformation|GetActorLocation _array_element)))
        (Variables|Default|SetOffsetZPosition (- (.z (Transformation|GetActorLocation _array_element)) 3e+02)))))
  (CallFunction|SinkChunkSet (stale Custom|Qeue%20Ice%20Chunk%20Set Active%20Chunk%20Set)))

(event Custom|Break%20Center%20Chunk
  ;[0 0 0] Separate events for separate ice sets
  (CallFunction|QeueIceChunkSet (Variables|Chunks|GetCenterIceChunk)))

(event Custom|Break%20Mid%20Ice%20Chunks
  ;[0 0 0] Separate events for separate ice sets
  (CallFunction|QeueIceChunkSet (Variables|Chunks|GetMidIceChunks)))

(event Custom|Break%20All%20Chunks
  ;[0 0 0] Separate events for separate ice sets
  (CallFunction|QeueIceChunkSet (Variables|Chunks|GetAllIceChunks)))

(event Custom|BreakSomeIce
  (bind _daref (Variables|Core|GetDARef))
  (bind _1steventtime (Variables|/Game/Blueprints/PDA/PDA_IceChunkManager.PDA_IceChunkManager_C|Get1stEventTime _daref))
  (bind _3rdeventtime (Variables|/Game/Blueprints/PDA/PDA_IceChunkManager.PDA_IceChunkManager_C|Get3rdEventTime _daref))
  (bind _2ndeventtime (Variables|/Game/Blueprints/PDA/PDA_IceChunkManager.PDA_IceChunkManager_C|Get2ndEventTime _daref))
  ;[0 0 0] Activate events depending on DA
  (if (<= (Variables|Core|GetEventIndex) 3)
    (Utilities|Time|SetTimerbyEvent (Utilities|Select :Index (Utilities|Array|Get(acopy) (Variables|/Game/Blueprints/PDA/PDA_IceChunkManager.PDA_IceChunkManager_C|GetEventIndex (Variables|Core|GetDARef)) (Variables|Core|GetEventIndex)) :NewEnumerator0 (EventDispatchers|CreateEvent :!event Custom|Break%20Edges) :NewEnumerator1 (EventDispatchers|CreateEvent :!event Custom|Break%20Center%20Chunk) :NewEnumerator2 (EventDispatchers|CreateEvent :!event Custom|Break%20Mid%20Ice%20Chunks) :NewEnumerator3 (EventDispatchers|CreateEvent :!event Custom|Break%20All%20Chunks)) (Utilities|Select :Index (Variables|Core|GetEventIndex) :Option%200 (- _1steventtime (Variables|/Game/Blueprints/PDA/PDA_IceChunkManager.PDA_IceChunkManager_C|GetStartTutorialTime _daref)) :Option%201 (- _2ndeventtime _1steventtime) :Option%202 (- _3rdeventtime _2ndeventtime) :Option%203 (- (Variables|/Game/Blueprints/PDA/PDA_IceChunkManager.PDA_IceChunkManager_C|GetFinalEventTime _daref) _3rdeventtime)))
    (Math|Integer|IncrementInt (Variables|Core|GetEventIndex))))

(event EventBeginPlay
  (bind _daref (Variables|Core|GetDARef))
  ;[0 0 0] Activate events depending on DA
  (Variables|Core|SetBreakingSignMaterial (Variables|/Game/Blueprints/PDA/PDA_IceChunkManager.PDA_IceChunkManager_C|GetBreakingSignMaterial _daref))
  (Variables|Core|SetOriginal%20Material (Variables|/Game/Blueprints/PDA/PDA_IceChunkManager.PDA_IceChunkManager_C|GetOriginalMaterial _daref))
  (Utilities|Time|SetTimerbyEvent (delegate Custom|BreakSomeIce) (Variables|/Game/Blueprints/PDA/PDA_IceChunkManager.PDA_IceChunkManager_C|GetStartTutorialTime (Variables|Core|GetDARef))))

(fn ConstructionScript)

(fn LightUpRandomIceChunk
  (if (> (Utilities|Array|Length (Variables|Chunks|GetAllIceChunks)) 1)
    (bind _output_get (Variables|Core|SetActiveChunk (Utilities|Array|Get(acopy) (Variables|Chunks|GetAllIceChunks) (Math|Random|RandomIntegerinRange 0 (- (Utilities|Array|Length (Variables|Chunks|GetAllIceChunks)) 1)))))
    (Rendering|Material|SetMaterial (Variables|/Script/Engine.StaticMeshActor|GetStaticMeshComponent _output_get) 0 (Variables|Core|GetBreakingSignMaterial))
    (Utilities|Array|AddUnique (Variables|Unused|GetIceChunksToDestroy) _output_get)
    (Utilities|Array|RemoveItem (Variables|Chunks|GetAllIceChunks) _output_get)
    (else
      (bind _output_get_2 (Variables|Core|SetActiveChunk (Utilities|Array|Get(acopy) (Variables|Chunks|GetAllIceChunks))))
      (Rendering|Material|SetMaterial (Variables|/Script/Engine.StaticMeshActor|GetStaticMeshComponent _output_get_2) 0 (Variables|Core|GetBreakingSignMaterial))
      (Utilities|Array|AddUnique (Variables|Unused|GetIceChunksToDestroy) _output_get_2)
      (Utilities|Array|RemoveItem (Variables|Chunks|GetAllIceChunks) _output_get_2))))