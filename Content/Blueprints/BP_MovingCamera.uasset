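; BP_MovingCamera is an AI-moved pawn that wanders the level and periodically stops to fake taking a picture with a screen flash.
; It chains AI MoveTo calls to random reachable nearby points, with floating movement speed read from DatasMovingCamera.
; A timed flag lets the next successful arrival trigger the picture: a short pause, a WBP_Flash widget on the viewport, then the cycle restarts.
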(event Custom|Move
  (bind _output_get (Variables|Default|SetRandomLocation (.RandomLocation (AI|Navigation|GetRandomReachablePointinRadius (Transformation|GetActorLocation) 1e+03 0 0))))
  (AI|AIMoveTo self _output_get 0 2e+01 false
    (:OnSuccess
      (if (Variables|Default|GetbTakePicture)
        (CallFunction|TakePicture)
        (else
          (CallFunction|Move))))
    (:OnFail
      (CallFunction|Move))))

(event Custom|WaitForPicture
  (Variables|Default|SetbTakePicture false)
  (CallFunction|Move)
  (Utilities|FlowControl|Delay 1e+01)
  (Variables|Default|SetbTakePicture true))

(event Custom|TakePicture
  (Utilities|FlowControl|Delay 1.5)
  (bind _returnvalue (UserInterface|CreateWidget "/Game/Blueprints/Widget/WBP_Flash.WBP_Flash_C"))
  (UserInterface|Viewport|AddtoViewport _returnvalue 0)
  (Utilities|FlowControl|Delay 1.0)
  (CallFunction|WaitforPicture))

(event EventBeginPlay
  (Variables|/Script/Engine.FloatingPawnMovement|SetMaxSpeed (Variables|Default|GetFloatingPawnMovement) (Variables|/Game/Blueprints/PDA/PDA_MovingCamera.PDA_MovingCamera_C|GetSpeed (Variables|Default|GetDatasMovingCamera)))
  (CallFunction|WaitforPicture))

(fn ConstructionScript)