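; BP_BreakingIce is a level actor, named as breaking ice, whose static mesh temporarily disappears after being hit.
; Any component hit swaps the mesh to a warning material and starts a configurable delay before it breaks.
; Breaking and respawning are done by setting the mesh's relative scale to zero, then back to one after a second delay.
; The original material is never restored.
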(event OnComponentHit(StaticMesh)
  (params (HitComponent :type Primitive%20Component%20Object%20Reference) (OtherActor :type Actor%20Object%20Reference) (OtherComp :type Primitive%20Component%20Object%20Reference) (NormalImpulse :type Vector :default "0, 0, 0") (Hit :type Hit%20Result%20Structure%20%28by%20ref%29))
  (Rendering|Material|SetMaterial (Variables|Default|GetStaticMesh) 0 (Variables|Default|GetBreakingSignMaterial))
  (Utilities|FlowControl|Delay (Variables|Default|GetDelayBeforeBreak))
  (Transformation|SetRelativeScale3D (Variables|Default|GetStaticMesh) "0, 0, 0")
  (Utilities|FlowControl|Delay (Variables|Default|GetDelayBeforeRespawn))
  (Transformation|SetRelativeScale3D (Variables|Default|GetStaticMesh) "1.000000,1.000000,1.000000"))

(event EventBeginPlay)

(event Collision|EventActorBeginOverlap
  (params (OtherActor :type Actor%20Object%20Reference)))

(event EventTick
  (params (DeltaSeconds :type Float%20%28single-precision%29)))

(fn ConstructionScript)