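; BP_BumpBush is a bush obstacle that knocks either of two local players back on overlap.
; It caches both BP_TiltedCharacter references when GM_Lumiere signals game start, then launches the overlapping player opposite their PunchArrow, scaled by PowerFactor, and plays a sound.
; A Feedback timeline scales the mesh for a bounce while the trigger sphere is shrunk to zero radius, preventing retriggers until it finishes.
; The construction script applies the configurable mesh and collision radius.
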(event OnComponentBeginOverlap(Sphere)
  (params (OverlappedComponent :type Primitive%20Component%20Object%20Reference) (OtherActor :type Actor%20Object%20Reference) (OtherComp :type Primitive%20Component%20Object%20Reference) (OtherBodyIndex :type Integer) (bFromSweep :type Boolean) (SweepResult :type Hit%20Result%20Structure%20%28by%20ref%29))
  ;[1 1 1] Checking for player
  (if (== OtherActor (Variables|Default|GetPlayer1Ref))
    (Variables|Default|SetCurrentPlayer (Variables|Default|GetPlayer1Ref))
    ;[1 1 1] Bouncing player back
    (Character|LaunchCharacter (Variables|Default|GetCurrentPlayer) (* (Math|Vector|GetForwardVector (Transformation|GetWorldRotation (Variables|/Game/Core/BP_Character.BP_Character_C|GetPunchArrow (Variables|Default|GetCurrentPlayer)))) (Variables|BounceVariables|GetpowerFactor) -1.0) true true :!label _label)
    ;[1 1 1] Play sound and FX
    (Audio|PlaySound2D 0 1.0 1.0 0.0 0 0)
    ;[1 1 1] Making the mesh bounce
    (Components|Sphere|SetSphereRadius (Variables|Default|GetSphere) 0.0 true)
    (bind _newtrack_0 (Timeline|Feedback PlayFromStart)
      (:Update
        (Transformation|SetRelativeScale3D (Variables|Default|GetMesh) (* (Variables|BounceVariables|GetBumpScaleUp) _newtrack_0)))
      (:Finished
        (Components|Sphere|SetSphereRadius (Variables|Default|GetSphere) (Variables|BounceVariables|GetCollisionRadius) true)
        (Transformation|SetRelativeScale3D (Variables|Default|GetMesh) "1.000000,1.000000,1.000000")))
    (elif (== OtherActor (Variables|Default|GetPlayer2Ref))
      (Variables|Default|SetCurrentPlayer (Variables|Default|GetPlayer2Ref))
      (goto _label))))

(event Custom|GetPlayerRef
  (bind _asbp_tilted_character (Utilities|Casting|CastToBP_TiltedCharacter (Game|GetPlayerCharacter 0)))
  (Variables|Default|SetPlayer1Ref _asbp_tilted_character)
  (bind _asbp_tilted_character_2 (Utilities|Casting|CastToBP_TiltedCharacter (Game|GetPlayerCharacter 1)))
  (Variables|Default|SetPlayer2Ref _asbp_tilted_character_2))

(event EventBeginPlay
  (bind _asgm_lumiere (Utilities|Casting|CastToGM_Lumiere (Game|GetGameMode)))
  (EventDispatchers|BindEventtoGameStart _asgm_lumiere (delegate Custom|GetPlayerRef)))

(event Collision|EventActorBeginOverlap
  (params (OtherActor :type Actor%20Object%20Reference)))

(event EventTick
  (params (DeltaSeconds :type Float%20%28single-precision%29)))

(fn ConstructionScript
  (Components|StaticMesh|SetStaticMesh (Variables|Default|GetMesh) (Variables|Mesh|GetBushMesh))
  (Components|Sphere|SetSphereRadius (Variables|Default|GetSphere) (Variables|BounceVariables|GetCollisionRadius) true))