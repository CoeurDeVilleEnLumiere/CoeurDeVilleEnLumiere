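; BP_TramLight is a tram light that blinks two lights, LightA and LightB, alternately from BeginPlay.
; Chained timer events swap the on and off materials between the lights, each step waiting Delay.
; After each full cycle it checks StillGoing, either restarting the sequence or setting both lights to the off material.
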(event Custom|ActivateLight_Event
  (Rendering|Material|SetMaterial (Variables|Default|GetLightA) 0 (Variables|Default|GetOnMaterial))
  (Rendering|Material|SetMaterial (Variables|Default|GetLightB) 0 (Variables|Default|GetOffMaterial))
  (Utilities|Time|SetTimerbyEvent (delegate Custom|SwitchLight) (Variables|Default|GetDelay)))

(event Custom|ExitOrRestart
  (if (Variables|Default|GetStillGoing)
    (CallFunction|ActivateLightEvent)
    (else
      (CallFunction|TurnOffLights))))

(event Custom|SwitchLight
  (Rendering|Material|SetMaterial (Variables|Default|GetLightB) 0 (Variables|Default|GetOnMaterial))
  (Rendering|Material|SetMaterial (Variables|Default|GetLightA) 0 (Variables|Default|GetOffMaterial))
  (Utilities|Time|SetTimerbyEvent (delegate Custom|ExitOrRestart) (Variables|Default|GetDelay)))

(event Custom|TurnOffLights
  (Rendering|Material|SetMaterial (Variables|Default|GetLightA) 0 (Variables|Default|GetOffMaterial))
  (Rendering|Material|SetMaterial (Variables|Default|GetLightB) 0 (Variables|Default|GetOffMaterial)))

(event EventBeginPlay
  (CallFunction|ActivateLightEvent))

(fn ConstructionScript)