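; BP_SaveSystem holds a PlayerScores list of records with usernames, with helpers to query and trim it.
; HasName scans the list and returns whether any entry's Username matches the given name.
; CheckPlayerScoreSize loops while the list exceeds 99 entries, removing index 0 and then index 1 each pass.
; Because indices shift after the first removal, each pass drops the original first and third entries.
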(fn HasName
  (params (name :type String))
  (for _array_element (Variables|Default|GetplayerScores)
    (if (Utilities|Enum|Equal(Enum) (.username _array_element) name)
      (return true)))
  (return false))

(fn CheckPlayerScoreSize
  (bind _playerscores (Variables|Default|GetplayerScores))
  (bind _returnvalue (Utilities|Array|Length _playerscores))
  (bind _returnvalue_2 (> _returnvalue 99))
  (while _returnvalue_2
    (if _returnvalue_2
      (Utilities|Array|RemoveIndex _playerscores)
      (Utilities|Array|RemoveIndex _playerscores 1))))