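; GM_Lumiere is the game mode for two-player local rounds, running each level from setup to transition.
; BeginPlay caches game instance, picture camera and item data, creates the second player, then after a delay shows the round widget, starts music and signals game start.
; ChoosePlayerStart assigns player indices and matches tagged starts.
; EndOfGame saves the camera's pictures, then async-loads the next level or shows the final HUD screen after level index 3.
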(event Custom|StartGame
  ;[1 1 1] Gameplay Start
  (Default|GetCurrentLevel (Variables|Ref|GetGI_LumiereRef))
  (bind _returnvalue (UserInterface|CreateWidget "/Game/Blueprints/Widget/WBP_Round.WBP_Round_C"))
  (UserInterface|Viewport|AddtoViewport _returnvalue 0)
  (Audio|PlaySound2D "/Game/Audio/Musics/Placeholder_CVLMusic_V1.Placeholder_CVLMusic_V1" 1.0 1.0 0.0 0 0)
  (Default|CallGameStart))

(event Custom|EndOfGame
  (bind _gi_lumiereref (Variables|Ref|GetGI_LumiereRef))
  (bind _currentlevel (Variables|/Game/Core/GI_Lumiere.GI_Lumiere_C|GetCurrentLevel _gi_lumiereref))
  (bind _levelsref (Variables|/Game/Core/GI_Lumiere.GI_Lumiere_C|GetLevelsRef _gi_lumiereref))
  (bind _returnvalue (+ _currentlevel 1))
  (bind _output (Utilities|Array|Get(acopy) _levelsref _returnvalue))
  ;[1 1 1] End Of Game
  (bind _returnvalue_2 (UserInterface|CreateWidget "/Game/Blueprints/Widget/WBP_LoadingScreen.WBP_LoadingScreen_C"))
  (UserInterface|Viewport|AddtoViewport _returnvalue_2 0)
  (Default|SaveAllPictures (Variables|Ref|GetPictureCameraRef))
  (Default|CallEndGame)
  (if (!= _currentlevel 3)
    (Utilities|AsyncLoadAsset _output
      (:Completed
        (Game|OpenLevel(byObjectReference) _output)))
    (else
      (Utilities|FlowControl|Delay 1.0)
      (Default|ShowEndOfGame (.AsHUD%20Lumiere (Utilities|Casting|CastToHUD_Lumiere (HUD|GetHUD (Game|GetPlayerController 0))))))))

(event Custom|SetUpPlayers
  ;[1 1 1] Set Up Players (index and outline)
  (for _index (range 0 1)
    (Default|SetUpCharacters (.AsPC%20Lumiere (Utilities|Casting|CastToPC_Lumiere (Game|GetPlayerController _index))))
    (Input|SetInputModeGameOnly (Game|GetPlayerController 0) false)
    (Input|SetInputModeGameOnly (Game|GetPlayerController 1) false)))

(event EventBeginPlay
  (bind _datasround (Variables|Datas|GetDatasRound))
  (bind _delaybeforegamestart (Variables|/Game/Blueprints/PDA/PDA_Round.PDA_Round_C|GetDelayBeforeGameStart _datasround))
  ;[1 1 1] Begin Play
  (bind _asgi_lumiere (Utilities|Casting|CastToGI_Lumiere (Game|GetGameInstance)))
  (Variables|Ref|SetGI_LumiereRef _asgi_lumiere)
  (bind _returnvalue (Actor|GetActorOfClass "/Game/Blueprints/Camera/BP_PictureCamera.BP_PictureCamera_C"))
  (Variables|Ref|SetPictureCameraRef _returnvalue)
  (Variables|Default|SetNumberOfItems (Variables|/Game/Blueprints/PDA/PDA_Item.PDA_Item_C|GetNumberOfItemToSpawn (Variables|Datas|GetDatasItems)))
  (Variables|Default|SetItemsCanSpawn (Variables|/Game/Blueprints/PDA/PDA_Item.PDA_Item_C|GetAllItems (Variables|Datas|GetDatasItems)))
  (Class|GameplayStatics|CreatePlayer 1)
  (CallFunction|SetUpPlayers)
  (Development|PrintString "BEFORE DELAY")
  (Development|PrintString (Utilities|String|ToString(Float) _delaybeforegamestart))
  (Utilities|FlowControl|Delay _delaybeforegamestart)
  (CallFunction|StartGame)
  (Utilities|FlowControl|Delay 0.2))

(fn ConstructionScript)

(fn ChoosePlayerStart
  (params (Player :type Controller%20Object%20Reference))
  (bind _aspc_lumiere (Utilities|Casting|CastToPC_Lumiere Player))
  (bind _output_get (Variables|Default|SetPlayerStartIndex (+ (Variables|Default|GetPlayerStartIndex) 1)))
  (Variables|/Game/Core/PC_Lumiere.PC_Lumiere_C|SetPlayerIndex _aspc_lumiere _output_get)
  (bind _outactors (Actor|GetAllActorsOfClass "/Script/Engine.PlayerStart"))
  (for _array_element _outactors
    (if (== (Variables|/Script/Engine.PlayerStart|GetPlayerStartTag _array_element) (Utilities|Select :Index (Variables|Default|GetPlayerStartIndex) :Option%200 "Player1" :Option%201 "Player2"))
      (return _array_element))))