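; GM_Lumiere is a game mode that sets up two-player local play when the level begins.
; It spawns a BP_Character at the first PlayerStart found and has player controller 0 possess it.
; It then creates a second local player, spawns another BP_Character at the second PlayerStart and has that new controller possess it.
; Leftover player-creation loop and input mapping context nodes are disconnected and never run.
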(event EventBeginPlay
  (bind _returnvalue (Game|GetPlayerController 0))
  (bind _outactors (Actor|GetAllActorsOfClass "/Script/Engine.PlayerStart"))
  (Utilities|FlowControl|Sequence
    (:then_0
      (bind _returnvalue_2 (Game|SpawnActorfromClass "/Game/Blueprint/GameMode/BP_Character.BP_Character_C" (Transformation|GetActorTransform (Utilities|Array|Get(acopy) _outactors)) "Undefined" "MultiplyWithRoot" _returnvalue 0))
      (Pawn|Possess _returnvalue _returnvalue_2))
    (:then_1
      (bind _returnvalue_3 (Class|GameplayStatics|CreatePlayer -1))
      (bind _returnvalue_4 (Game|SpawnActorfromClass "/Game/Blueprint/GameMode/BP_Character.BP_Character_C" (Transformation|GetActorTransform (Utilities|Array|Get(acopy) _outactors 1)) "Undefined" "MultiplyWithRoot" _returnvalue_3 0))
      (Pawn|Possess _returnvalue_3 _returnvalue_4))))

(fn ConstructionScript)